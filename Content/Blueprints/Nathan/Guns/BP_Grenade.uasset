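; BP_Grenade is a grenade actor that deals area damage on impact and then destroys itself.
; When its Sphere component hits another actor, a multi-sphere trace at its location gathers WorldDynamic and Pawn objects within Radius, with debug drawing on.
; Each trace hit triggers a separate radial damage call at its impact point, so overlapping damage can stack, and names the hit actor as damage causer.
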(event `self.Sphere.OnComponentHit`
  (params (HitComponent :type "PrimitiveComponent Object Reference") (OtherActor :type "Actor Object Reference") (OtherComp :type "PrimitiveComponent Object Reference") (NormalImpulse :type "Vector Structure") (Hit :type "HitResult Structure (by ref)"))
  (bind _returnvalue (`self.K2_GetActorLocation`))
  (if (not (== OtherActor self))
    (bind _outhits (`KismetSystemLibrary.SphereTraceMultiForObjects` _returnvalue (+ _returnvalue (0.0 0.0 0.1)) (`self.Radius`) (`|MakeArray` "ObjectTypeQuery2" "ObjectTypeQuery3" :!type "EObjectTypeQuery Enum") false (`|MakeArray` self :!type "Actor Object Reference") "ForDuration"))
    (for _array_element _outhits
      (bind (_bblockinghit _binitialoverlap _time _distance _location _impactpoint _normal _impactnormal _physmat _hitactor) (`GameplayStatics.BreakHitResult` _array_element))
      (`GameplayStatics.ApplyRadialDamage` (`self.Base Damage`) _impactpoint (`self.Radius`) null (`|MakeArray` self :!type "Actor Object Reference") _hitactor null))
    (`self.K2_DestroyActor`)))

(fn `UserConstructionScript`)
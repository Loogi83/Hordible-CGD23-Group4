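; Test player character with movement, look, sprint, crouch, jump, a switchable five-weapon inventory and a melee attack.
; Weapons are child actor components, cycled by mouse wheel with wraparound, and Equipped shows only the current one.
; Left click calls Attack on the current weapon and clears its timer on release, while a Bow flag switches to charge-and-release on the level's bow actor.
; Melee applies damage through a short camera line trace with debug drawing.
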(event `Key|LeftMouseButton`
  (params (Key :type "Key Structure"))
  (bind _bow (`self.Bow`))
  ;[1 0 0.01752] Attack using equipped Gun
  (:`Pressed`
    (if _bow
      (bind _returnvalue (`GameplayStatics.GetActorOfClass` "/Game/Blueprints/Nathan/Guns/WeaponBow_BPC.WeaponBow_BPC_C"))
      (`/Game/Blueprints/Nathan/Guns/WeaponBow_BPC.Charged Shot` _returnvalue)
      (else
        (bind _asbase_weapon_bpp (cast `/Game/Blueprints/Nathan/Guns/BaseWeapon_BPP` (`ChildActorComponent.ChildActor` (`|GetArrayItem` (`self.Gun Inventory`) (`self.Current Weapon`)))))
        (`/Game/Blueprints/Nathan/Guns/BaseWeapon_BPP.Attack` _asbase_weapon_bpp))))
  (:`Released`
    (if _bow
      (`/Game/Blueprints/Nathan/Guns/BaseWeapon_BPP.Attack` _returnvalue)
      (else
        (`KismetSystemLibrary.K2_ClearAndInvalidateTimerHandle` (`/Game/Blueprints/Nathan/Guns/BaseWeapon_BPP.Gun Timer Ref` _asbase_weapon_bpp))))))

(event `InputAxisKey|MouseWheelAxis`
  (params (AxisValue :type "Float (single-precision)"))
  (bind _gun_inventory (`self.Gun Inventory`))
  (bind _returnvalue (+ (`KismetMathLibrary.FTrunc` AxisValue) (`self.Current Weapon`)))
  ;[0.4072 0 0.2384] Weapon Switching System
  (if (`KismetArrayLibrary.Array_IsValidIndex` (`self.Gun Inventory`) _returnvalue)
    (set `self.Current Weapon` _returnvalue)
    (`self.Equipped` _gun_inventory)
    (elif (< _returnvalue 0)
      (set `self.Current Weapon` (`KismetArrayLibrary.Array_LastIndex` (`self.Gun Inventory`)))
      (`self.Equipped` _gun_inventory)
      (else
        (set `self.Current Weapon` 0)
        (`self.Equipped` _gun_inventory)
        (set `self.Bow` (== (`ChildActorComponent.ChildActor` (`|GetArrayItem` (`self.Gun Inventory`) (`self.Current Weapon`))) (`self.Gun3`)))))))

(event `self.ReceiveBeginPlay`
  ;[1 0 0.587] Set Up Gun Inventory and Equip First Gun
  (bind _output_get (set `self.Gun Inventory` (`|MakeArray` (`self.Gun`) (`self.Gun1`) (`self.Gun2`) (`self.Gun3`) (`self.Gun4`))))
  (`self.Equipped` _output_get))

(event `InputAction|Crouch`
  (params (Key :type "Key Structure"))
  ;[0 1 0.003621] Movement
  (:`Pressed`
    (`self.Crouch`))
  (:`Released`
    (`self.UnCrouch`)))

(event `InputAction|Run`
  (params (Key :type "Key Structure"))
  (bind _charactermovement (`self.CharacterMovement`))
  ;[0 1 0.003621] Movement
  (:`Pressed`
    (set `CharacterMovementComponent.MaxWalkSpeed` (`self.runSpeed`) _charactermovement))
  (:`Released`
    (set `CharacterMovementComponent.MaxWalkSpeed` (`self.walkSpeed`) _charactermovement)))

(event `InputAxis|MoveForward`
  (params (AxisValue :type "Float (single-precision)"))
  ;[0 1 0.003621] Movement
  (`PawnMovementComponent.AddInputVector` (`self.CharacterMovement`) (* AxisValue (`self.GetActorForwardVector`)) false))

(event `InputAction|Jump`
  (params (Key :type "Key Structure"))
  ;[0 1 0.003621] Movement
  (:`Pressed`
    (`self.Jump`)))

(event `InputAxis|MoveRight`
  (params (AxisValue :type "Float (single-precision)"))
  ;[0 1 0.003621] Movement
  (`PawnMovementComponent.AddInputVector` (`self.CharacterMovement`) (* AxisValue (`self.GetActorRightVector`)) false))

(event `InputAxis|LookUp`
  (params (AxisValue :type "Float (single-precision)"))
  ;[0.955 1 0] Look
  (`self.AddControllerPitchInput` AxisValue))

(event `InputAxis|LookRight`
  (params (AxisValue :type "Float (single-precision)"))
  ;[0.955 1 0] Look
  (`self.AddControllerYawInput` AxisValue))

(event `InputAction|Melee`
  (params (Key :type "Key Structure"))
  (bind _returnvalue (`SceneComponent.K2_GetComponentLocation` (`self.Camera`)))
  ;[0 0.8833 1] Melee Attack
  (:`Pressed`
    (bind _outhit (`KismetSystemLibrary.LineTraceSingle` :`Start` _returnvalue :`End` (+ _returnvalue (* (`KismetMathLibrary.GetForwardVector` (`Controller.GetControlRotation` (`GameplayStatics.GetPlayerController` 0))) 200.0)) :`TraceChannel` "TraceTypeQuery1" :`DrawDebugType` "ForDuration"))
    (`GameplayStatics.ApplyDamage` (`.HitActor` (`GameplayStatics.BreakHitResult` _outhit)) 2.0)))

(fn `Equipped`
  (params (Array :type "Array of ChildActorComponent Object Reference"))
  (for _array_element Array
    (`SceneComponent.SetVisibility` _array_element false false))
  (`SceneComponent.SetVisibility` (`|GetArrayItem` Array (`self.Current Weapon`)) true false))

(fn `UserConstructionScript`)
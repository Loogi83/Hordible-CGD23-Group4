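; BP_Bloblin is an enemy that splits into smaller Bloblet enemies when it dies.
; Its Death override spawns a configurable number of BP_Bloblet actors at its own transform, launching each valid one upward with a random horizontal push so they scatter.
; It then calls the parent Death; the event graph and construction script add no logic of their own.
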(fn `Death`
  (bind _returnvalue (`KismetMathLibrary.RandomFloatInRange` -200.0 200.0))
  (bind (_returnvalue_location _returnvalue_rotation) (`KismetMathLibrary.BreakTransform` (`self.GetTransform` self)))
  ;[1 1 1] spawns x number of enemies at Bloblin location on death
  (for _ (range 1 (+ (`self.NumberOfEnemiesToSpawn`) 1))
    (bind _returnvalue_2 (`|SpawnActorFromClass` "/Game/Blueprints/Kieran/Enemies/BP_Bloblet.BP_Bloblet_C" (`KismetMathLibrary.MakeTransform` _returnvalue_location _returnvalue_rotation) "Undefined" "OverrideRootScale" null null))
    (`/Engine/EditorBlueprintResources/StandardMacros.IsValid` _returnvalue_2
      (:`Is Valid`
        (`self.LaunchCharacter` _returnvalue_2 (`KismetMathLibrary.MakeVector` _returnvalue _returnvalue 200.0) false false))))
  (`parent.Death`))

(fn `UserConstructionScript`
  (`parent.UserConstructionScript`))
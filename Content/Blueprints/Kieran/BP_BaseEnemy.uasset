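; Base enemy character Blueprint that holds health and movement stats in an enemy stats struct and handles taking damage and death.
; The construction script sets current health to max and applies the struct's movement speed to the character movement component.
; The DamageEnemy event subtracts health, then broadcasts an enemy-killed dispatcher and destroys the actor at zero.
; Tick draws current health above the enemy as debug text.
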(event `/Game/Blueprints/Kieran/BPI_DamageEnemy.DamageEnemy`
  (params (DamageToDeal :type "Float (double-precision)"))
  (`self.TakeDamage` DamageToDeal))

(event `self.ReceiveTick`
  (params (DeltaSeconds :type "Float (single-precision)"))
  (`KismetSystemLibrary.DrawDebugString` (0.0 0.0 100.0) (`KismetStringLibrary.Conv_DoubleToString` (`.CurrentHealth_4_84644DB54A34569CA27C329BDE205092` (break `/Game/Blueprints/Kieran/S_EnemyStats` (`self.Stats`)))) self))

(fn `TakeDamage`
  (params (DamageDealt :type "Float (double-precision)"))
  (bind (_movementspeed _currenthealth) (break `/Game/Blueprints/Kieran/S_EnemyStats` (`self.Stats`)))
  (setmembers `/Game/Blueprints/Kieran/S_EnemyStats` :`StructRef` (`self.Stats`) :`CurrentHealth` (- _currenthealth DamageDealt))
  (if (<= _currenthealth 0.0)
    (`self.EEnemyKilled`)
    (`self.K2_DestroyActor`)))

(fn `UserConstructionScript`
  (bind _stats (`self.Stats`))
  (bind ((`MovementSpeed_2_28FA2C6348DBB2A1392799B2F3D03407` _movementspeed) (`MaxHealth_6_D9738A614FE71AD569592B8B8F0B25C8` _maxhealth)) (break `/Game/Blueprints/Kieran/S_EnemyStats` _stats))
  ;[1 1 1] Sets current health to max (saves manually changing both stats)
  (setmembers `/Game/Blueprints/Kieran/S_EnemyStats` :`StructRef` _stats :`CurrentHealth` _maxhealth)
  ;[1 1 1] Sets character movement speed as struct variable
  (set `CharacterMovementComponent.MaxWalkSpeed` _movementspeed (`self.CharacterMovement`)))
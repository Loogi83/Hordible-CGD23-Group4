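; BP_PickupParent is a base pickup actor that hovers in place and is collected when something touches it.
; A Hover timeline starts on BeginPlay and lerps the static mesh's relative location between two stored points.
; The sphere's overlap event ignores BP_BaseEnemy actors and calls OnPickup for any other actor, which prints a debug string and destroys the pickup.
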(event `self.ReceiveBeginPlay`
  (bind (_direction _alpha) (`Timeline|Hover` :!via `PlayFromStart`)
    (:`Update`
      (`SceneComponent.K2_SetRelativeLocation` (`self.StaticMesh`) (`KismetMathLibrary.VLerp` (`self.locationA`) (`self.locationB`) _alpha) false false))))

(event `self.Sphere.OnComponentBeginOverlap`
  (params (OverlappedComponent :type "PrimitiveComponent Object Reference") (OtherActor :type "Actor Object Reference") (OtherComp :type "PrimitiveComponent Object Reference") (OtherBodyIndex :type Integer) (bFromSweep :type Boolean) (SweepResult :type "HitResult Structure (by ref)"))
  (cast `/Game/Blueprints/Kieran/Enemies/BP_BaseEnemy` OtherActor
    (:`CastFailed`
      (`self.onPickup`))))

(fn `onPickup`
  (`KismetSystemLibrary.PrintString` "PickedUp")
  (`self.K2_DestroyActor`))

(fn `UserConstructionScript`)
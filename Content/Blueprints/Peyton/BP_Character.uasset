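; Player character Blueprint that handles walk, run, crouch, jump, look and simple hitscan attacks.
; Movement inputs feed CharacterMovement and look inputs turn the controller, with run toggling max speed from the WalkSpeed set in the construction script.
; Left click fires MeleeAttack, a short debug-drawn line trace from the camera along player 0's control rotation that damages the hit actor.
; RangedAttack repeats this with longer reach and higher damage, but nothing here calls it.
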(event `InputAction|Crouch`
  (params (Key :type "Key Structure"))
  ;[0 1 0.003621] Movement
  (:`Pressed`
    (`self.Crouch`))
  (:`Released`
    (`self.UnCrouch`)))

(event `InputAction|Run`
  (params (Key :type "Key Structure"))
  (bind _charactermovement (`self.CharacterMovement`))
  ;[0 1 0.003621] Movement
  (:`Pressed`
    (set `CharacterMovementComponent.MaxWalkSpeed` (`self.runSpeed`) _charactermovement))
  (:`Released`
    (set `CharacterMovementComponent.MaxWalkSpeed` (`self.walkSpeed`) _charactermovement)))

(event `InputAxis|MoveForward`
  (params (AxisValue :type "Float (single-precision)"))
  ;[0 1 0.003621] Movement
  (`PawnMovementComponent.AddInputVector` (`self.CharacterMovement`) (* AxisValue (`self.GetActorForwardVector`)) false))

(event `InputAction|Jump`
  (params (Key :type "Key Structure"))
  ;[0 1 0.003621] Movement
  (:`Pressed`
    (`self.Jump`)))

(event `InputAxis|MoveRight`
  (params (AxisValue :type "Float (single-precision)"))
  ;[0 1 0.003621] Movement
  (`PawnMovementComponent.AddInputVector` (`self.CharacterMovement`) (* AxisValue (`self.GetActorRightVector`)) false))

(event `InputAxis|LookUp`
  (params (AxisValue :type "Float (single-precision)"))
  ;[0.955 1 0] Look
  (`self.AddControllerPitchInput` AxisValue))

(event `InputAxis|LookRight`
  (params (AxisValue :type "Float (single-precision)"))
  ;[0.955 1 0] Look
  (`self.AddControllerYawInput` AxisValue))

(event `Key|LeftMouseButton`
  (params (Key :type "Key Structure"))
  (:`Pressed`
    (`self.Melee Attack`)))

(event `Melee Attack`
  (bind _returnvalue (`SceneComponent.K2_GetComponentLocation` (`self.Camera`)))
  (bind _outhit (`KismetSystemLibrary.LineTraceSingle` :`Start` _returnvalue :`End` (+ _returnvalue (* (`KismetMathLibrary.GetForwardVector` (`Controller.GetControlRotation` (`GameplayStatics.GetPlayerController` 0))) 200.0)) :`TraceChannel` "TraceTypeQuery1" :`DrawDebugType` "ForDuration"))
  (`GameplayStatics.ApplyDamage` (`.HitActor` (`GameplayStatics.BreakHitResult` _outhit)) 2.0))

(event `Ranged Attack`
  (bind _returnvalue (`SceneComponent.K2_GetComponentLocation` (`self.Camera`)))
  (bind _outhit (`KismetSystemLibrary.LineTraceSingle` :`Start` _returnvalue :`End` (+ _returnvalue (* (`KismetMathLibrary.GetForwardVector` (`Controller.GetControlRotation` (`GameplayStatics.GetPlayerController` 0))) 500.0)) :`TraceChannel` "TraceTypeQuery1" :`DrawDebugType` "ForDuration"))
  (`GameplayStatics.ApplyDamage` (`.HitActor` (`GameplayStatics.BreakHitResult` _outhit)) 5.0))

(fn `UserConstructionScript`
  (set `CharacterMovementComponent.MaxWalkSpeed` (`self.walkSpeed`) (`self.CharacterMovement`)))
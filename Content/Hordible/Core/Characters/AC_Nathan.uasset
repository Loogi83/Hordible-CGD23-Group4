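; AC_Nathan is the player's weapon component, managing an inventory of child-actor guns and handling switching and firing.
; Init equips the starting gun, and Add events append pistol, crossbow, shotgun or grenade launcher if unlocked, saving each index and equipping it.
; Number keys jump to saved indices and scrolling wraps through the array, with Equipped showing only the current gun.
; Attack input casts that gun's child actor to BaseWeapon_BPP to fire or cancel.
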(event `InputAction|Weapon1`
  (params (Key :type "Key Structure"))
  ;[0.1683 0 0.09759] Manual Switching of Weapons through Number Keybinds
  (:`Pressed`
    (set `self.Current Weapon` 0)
    (`self.Equipped` (`self.Gun Inventory`))))

(event `InputAction|Weapon2`
  (params (Key :type "Key Structure"))
  ;[0.1683 0 0.09759] Manual Switching of Weapons through Number Keybinds
  (:`Pressed`
    (if (`self.UnlockedPistol`)
      (set `self.Current Weapon` (`self.PistolNumber`))
      (`self.Equipped` (`self.Gun Inventory`)))))

(event `InputAction|Weapon3`
  (params (Key :type "Key Structure"))
  ;[0.1683 0 0.09759] Manual Switching of Weapons through Number Keybinds
  (:`Pressed`
    (if (`self.UnlockedCrossbow`)
      (set `self.Current Weapon` (`self.CrossbowNumber`))
      (`self.Equipped` (`self.Gun Inventory`)))))

(event `InputAction|Weapon4`
  (params (Key :type "Key Structure"))
  ;[0.1683 0 0.09759] Manual Switching of Weapons through Number Keybinds
  (:`Pressed`
    (if (`self.UnlockedGrenadeLauncher`)
      (set `self.Current Weapon` (`self.GLNumber`))
      (`self.Equipped` (`self.Gun Inventory`)))))

(event `InputAction|Weapon5`
  (params (Key :type "Key Structure"))
  ;[0.1683 0 0.09759] Manual Switching of Weapons through Number Keybinds
  (:`Pressed`
    (if (`self.UnlockedShotgun`)
      (set `self.Current Weapon` (`self.ShotgunNumber`))
      (`self.Equipped` (`self.Gun Inventory`)))))

(event `InputAction|Attack`
  (params (Key :type "Key Structure"))
  ;[1 0 0.01752] Attack using equipped Gun
  (:`Pressed`
    (`self.Start Fire`))
  (:`Released`
    (`self.Stop Fire`)))

(event `Start Fire`
  ;[1 0 0.01752] Attack using equipped Gun
  (bind _asbase_weapon_bpp (cast `/Game/Hordible/Core/Weapons/BaseWeapon_BPP` (`ChildActorComponent.ChildActor` (`|GetArrayItem` (`self.Gun Inventory`) (`self.Current Weapon`)))))
  (`/Game/Hordible/Core/Weapons/BaseWeapon_BPP.Attack` _asbase_weapon_bpp))

(event `Stop Fire`
  ;[1 0 0.01752] Attack using equipped Gun
  (bind _asbase_weapon_bpp (cast `/Game/Hordible/Core/Weapons/BaseWeapon_BPP` (`ChildActorComponent.ChildActor` (`|GetArrayItem` (`self.Gun Inventory`) (`self.Current Weapon`)))))
  (`/Game/Hordible/Core/Weapons/BaseWeapon_BPP.Cancel` _asbase_weapon_bpp))

(event `InputAxis|ScrollWeapons`
  (params (AxisValue :type "Float (single-precision)"))
  (bind _gun_inventory (`self.Gun Inventory`))
  (bind _returnvalue (+ (`KismetMathLibrary.FTrunc` AxisValue) (`self.Current Weapon`)))
  ;[0.4072 0 0.2384] Weapon Switching System
  (if (`KismetArrayLibrary.Array_IsValidIndex` (`self.Gun Inventory`) _returnvalue)
    (set `self.Current Weapon` _returnvalue)
    (`self.Equipped` _gun_inventory)
    (elif (< _returnvalue 0)
      (set `self.Current Weapon` (`KismetArrayLibrary.Array_LastIndex` (`self.Gun Inventory`)))
      (`self.Equipped` _gun_inventory)
      (else
        (set `self.Current Weapon` 0)
        (`self.Equipped` _gun_inventory)))))

(event `Init`
  (params (Gun :type "ChildActorComponent Object Reference") (Gun1 :type "ChildActorComponent Object Reference") (Gun2 :type "ChildActorComponent Object Reference") (Gun3 :type "ChildActorComponent Object Reference") (Gun4 :type "ChildActorComponent Object Reference"))
  ;[1 0 0.587] Set Up Gun Inventory and Equip First Gun
  (bind _output_get (set `self.Gun Inventory` (`|MakeArray` Gun)))
  (`self.Equipped` _output_get)
  (`self.CurrentWeapon`))

(event `AddPistol`
  (params (Pistol :type "ChildActorComponent Object Reference"))
  (bind _gun_inventory (`self.Gun Inventory`))
  ;[0.3813 0.03313 0.235] Adding Weapons to Gun Inventory
  (if (`self.UnlockedPistol`)
    (bind _returnvalue (`KismetArrayLibrary.Array_Add` _gun_inventory Pistol))
    (set `self.PistolNumber` _returnvalue)
    (set `self.Current Weapon` _returnvalue)
    (`SceneComponent.SetVisibility` Pistol true false)
    (`self.Equipped` _gun_inventory)))

(event `AddCrossbow`
  (params (Crossbow :type "ChildActorComponent Object Reference"))
  (bind _gun_inventory (`self.Gun Inventory`))
  ;[0.3813 0.03313 0.235] Adding Weapons to Gun Inventory
  (if (`self.UnlockedCrossbow`)
    (bind _returnvalue (`KismetArrayLibrary.Array_Add` _gun_inventory Crossbow))
    (set `self.CrossbowNumber` _returnvalue)
    (set `self.Current Weapon` _returnvalue)
    (`SceneComponent.SetVisibility` Crossbow true false)
    (`self.Equipped` _gun_inventory)))

(event `AddShotgun`
  (params (Shotgun :type "ChildActorComponent Object Reference"))
  (bind _gun_inventory (`self.Gun Inventory`))
  ;[0.3813 0.03313 0.235] Adding Weapons to Gun Inventory
  (if (`self.UnlockedShotgun`)
    (bind _returnvalue (`KismetArrayLibrary.Array_Add` _gun_inventory Shotgun))
    (set `self.ShotgunNumber` _returnvalue)
    (set `self.Current Weapon` _returnvalue)
    (`SceneComponent.SetVisibility` Shotgun true false)
    (`self.Equipped` _gun_inventory)))

(event `AddGrenadeLauncher`
  (params (GrenadeLauncher :type "ChildActorComponent Object Reference"))
  (bind _gun_inventory (`self.Gun Inventory`))
  ;[0.3813 0.03313 0.235] Adding Weapons to Gun Inventory
  (if (`self.UnlockedGrenadeLauncher`)
    (bind _returnvalue (`KismetArrayLibrary.Array_Add` _gun_inventory GrenadeLauncher))
    (set `self.GLNumber` _returnvalue)
    (set `self.Current Weapon` _returnvalue)
    (`SceneComponent.SetVisibility` GrenadeLauncher true false)
    (`self.Equipped` _gun_inventory)))

(fn `Equipped`
  (params (Array :type "Array of ChildActorComponent Object Reference"))
  (for _array_element Array
    (`SceneComponent.SetVisibility` _array_element false false))
  (`SceneComponent.SetVisibility` (`|GetArrayItem` Array (`self.Current Weapon`)) true false))
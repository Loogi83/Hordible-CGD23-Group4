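; Player character for Hordible, handling movement, sensitivity-scaled look, shield-bash melee, weapon recoil and pickups.
; ACNathan receives weapon meshes and unlocks, while ACKieran handles melee alongside a timeline that moves the Shield mesh.
; TakeDamage drains an active shield or health, drives the damage UI and death, and doubles as healing when DamagePlayer is false.
; Timed pickups grant shield, an invisibility material on Shield, and a double-points flag on GM_Wave.
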(event `/Game/Hordible/Core/Weapons/BPI_AddWeapons.GrenadeLauncher`
  (bind _ac_nathan (`self.AC_Nathan`))
  ;[0.8323 0 1] Pickup Events For adding Guns to Gun Inventory
  (set `/Game/Hordible/Core/Characters/AC_Nathan.UnlockedGrenadeLauncher` true _ac_nathan)
  (`/Game/Hordible/Core/Characters/AC_Nathan.AddGrenadeLauncher` _ac_nathan (`self.LauncherMesh`)))

(event `/Game/Hordible/Core/Weapons/BPI_AddWeapons.Crossbow`
  (bind _ac_nathan (`self.AC_Nathan`))
  ;[0.8323 0 1] Pickup Events For adding Guns to Gun Inventory
  (set `/Game/Hordible/Core/Characters/AC_Nathan.UnlockedCrossbow` true _ac_nathan)
  (`/Game/Hordible/Core/Characters/AC_Nathan.AddCrossbow` _ac_nathan (`self.CrossbowMesh`)))

(event `Damage Effect`
  (bind _healthcurrent (`self.HealthCurrent`))
  (bind _damageui (`self.DamageUI`))
  ;[1 0.2613 0] Activate the Damage Effect UI according to damage taken
  (set `self.EffectActive` true)
  (`UserWidget.AddToViewport` _damageui 0)
  (if (<= _healthcurrent 50.0)
    (`/Game/Hordible/Core/UI/WBP_BloodSplatter.CriticalHealth` _damageui)
    (elif (> _healthcurrent 50.0)
      (`/Game/Hordible/Core/UI/WBP_BloodSplatter.Damage` _damageui))))

(event `/Game/Hordible/Core/Weapons/BPI_AddWeapons.Shotgun`
  (bind _ac_nathan (`self.AC_Nathan`))
  ;[0.8323 0 1] Pickup Events For adding Guns to Gun Inventory
  (set `/Game/Hordible/Core/Characters/AC_Nathan.UnlockedShotgun` true _ac_nathan)
  (`/Game/Hordible/Core/Characters/AC_Nathan.AddShotgun` _ac_nathan (`self.ShotgunMesh`)))

(event `/Game/Hordible/Core/Weapons/BPI_AddWeapons.Pistol`
  (bind _ac_nathan (`self.AC_Nathan`))
  ;[0.8323 0 1] Pickup Events For adding Guns to Gun Inventory
  (set `/Game/Hordible/Core/Characters/AC_Nathan.UnlockedPistol` true _ac_nathan)
  (`/Game/Hordible/Core/Characters/AC_Nathan.AddPistol` _ac_nathan (`self.PistolMesh`)))

(event `self.ReceiveBeginPlay`
  ;[1 0.9017 0] Component Inits
  (`/Game/Hordible/Core/Characters/AC_Nathan.Init` (`self.AC_Nathan`) (`self.RifleMesh`) (`self.ShotgunMesh`) (`self.PistolMesh`) (`self.CrossbowMesh`) (`self.LauncherMesh`))
  (`/Game/Hordible/Core/Characters/AC_Kieran.Init` (`self.AC_Kieran`) (`self.Camera`))
  (set `self.Start Location` (`SceneComponent.RelativeLocation` (`self.Shield`)))
  (`KismetSystemLibrary.K2_SetTimerDelegate` (delegate `DirectionTick`) 0.05 true)
  (set `self.GameInstanceRef` (cast `/Game/Hordible/Core/GameModes/HordibleInstance` (`GameplayStatics.GetGameInstance`) :!pure true))
  (bind _returnvalue (`|CreateWidget` "/Game/Hordible/Core/UI/WBP_BloodSplatter.WBP_BloodSplatter_C"))
  (set `self.DamageUI` _returnvalue))

(event `DirectionTick`
  (bind _movementdirection (`self.MovementDirection`))
  (bind (_returnvalue_roll _returnvalue_pitch _returnvalue_yaw) (`KismetMathLibrary.BreakRotator` (`SceneComponent.K2_GetComponentRotation` _movementdirection)))
  ;[1 0.9017 0] Component Inits
  (`SceneComponent.K2_SetWorldRotation` _movementdirection (`KismetMathLibrary.MakeRotator` _returnvalue_roll 0.0 _returnvalue_yaw) false false))

(event `InputAction|Crouch`
  (params (Key :type "Key Structure"))
  ;[0 1 0.003621] Movement
  (:`Pressed`
    (`self.Crouch`))
  (:`Released`
    (`self.UnCrouch`)))

(event `InputAction|Run`
  (params (Key :type "Key Structure"))
  (bind _charactermovement (`self.CharacterMovement`))
  ;[0 1 0.003621] Movement
  (:`Pressed`
    (set `CharacterMovementComponent.MaxWalkSpeed` (`self.RunSpeed`) _charactermovement))
  (:`Released`
    (set `CharacterMovementComponent.MaxWalkSpeed` (`self.WalkSpeed`) _charactermovement)))

(event `InputAxis|MoveForward`
  (params (AxisValue :type "Float (single-precision)"))
  ;[0 1 0.003621] Movement
  (`PawnMovementComponent.AddInputVector` (`self.CharacterMovement`) (* AxisValue (`SceneComponent.GetForwardVector` (`self.MovementDirection`))) false))

(event `InputAction|Jump`
  (params (Key :type "Key Structure"))
  ;[0 1 0.003621] Movement
  (:`Pressed`
    (`self.Jump`)))

(event `InputAxis|MoveRight`
  (params (AxisValue :type "Float (single-precision)"))
  ;[0 1 0.003621] Movement
  (`PawnMovementComponent.AddInputVector` (`self.CharacterMovement`) (* AxisValue (`self.GetActorRightVector`)) false))

(event `self.ReceiveTick`
  (params (DeltaSeconds :type "Float (single-precision)"))
  (`KismetSystemLibrary.PrintString` (`KismetStringLibrary.Concat_StrStr` "Shield Active? = " (`KismetStringLibrary.Conv_BoolToString` (`self.ShieldActive`))) true true (struct :`G` 0.335926 :`B` 1.0 :`A` 1.0) 0.0))

(event `InputAxis|LookUp`
  (params (AxisValue :type "Float (single-precision)"))
  ;[0.955 1 0] Look
  (`self.AddControllerPitchInput` (* AxisValue (`/Game/Hordible/Core/GameModes/HordibleInstance.Sensitivity` (`self.GameInstanceRef`)))))

(event `InputAxis|LookRight`
  (params (AxisValue :type "Float (single-precision)"))
  ;[0.955 1 0] Look
  (`self.AddControllerYawInput` (* AxisValue (`/Game/Hordible/Core/GameModes/HordibleInstance.Sensitivity` (`self.GameInstanceRef`)))))

(event `/Game/Hordible/Placeables/Pickups/BPI_PickUp.PickupHealth`
  (params (Health :type "Float (double-precision)"))
  (bind _healthcurrent (`self.HealthCurrent`))
  (bind _healthmax (`self.HealthMax`))
  ;[0.2203 1 0] Add Health To player When Interface Activated
  (set `self.Damage Player` false)
  (if (>= (+ _healthcurrent Health) _healthmax)
    (set `self.HealthCurrent` _healthmax)
    (set `self.Damage Player` true)
    (elif (not (>= _healthcurrent _healthmax))
      (`self.TakeDamage` Health)
      (set `self.Damage Player` true))))

(event `InputAction|Melee`
  (params (Key :type "Key Structure"))
  (bind _start_location (`self.Start Location`))
  ;[1 0 0.04935] Shield Attack and Animation
  (:`Pressed`
    (if (`self.bCanMelee`)
      (set `self.bCanMelee` false)
      (`/Game/Hordible/Core/Characters/AC_Kieran.Melee Attack` (`self.AC_Kieran`))
      (`ActorComponent.Activate` (`self.NS_ShieldBash`) true)
      (`ActorComponent.Activate` (`self.NS_ShieldBash1`) true)
      (`ActorComponent.Activate` (`self.NS_ShieldBash2`) true)
      (bind (_direction _bash) (`Timeline|Shield Bash` :!via `PlayFromStart`)
        (:`Update`
          (`SceneComponent.K2_SetRelativeLocation` (`self.Shield`) (`KismetMathLibrary.VLerp` _start_location (+ _start_location (`self.ShieldLocation`)) _bash) false false))
        (:`Finished`
          (set `self.bCanMelee` true))))))

(event `/Game/Hordible/Core/Characters/BPI_DamagePlayer.DamagePlayer`
  (params (Value :type "Float (double-precision)"))
  (`self.TakeDamage` Value))

(event `/Game/Hordible/Placeables/Pickups/BPI_PickUp.PickupDoublePoints`
  ;[1 1 1] Set effect to active in game mode
  (bind _asgm_wave (cast `/Game/Hordible/Core/GameModes/GM_Wave` (`GameplayStatics.GetGameMode`)))
  (set `/Game/Hordible/Core/GameModes/GM_Wave.Effect Active` true _asgm_wave)
  (`KismetSystemLibrary.Delay` 10.0)
  (set `/Game/Hordible/Core/GameModes/GM_Wave.Effect Active` false _asgm_wave))

(event `/Game/Hordible/Placeables/Pickups/BPI_PickUp.PickupShield`
  (params (Shield :type "Float (double-precision)"))
  ;[1 1 1] Add Shield To Player When Interface Activated
  (set `self.ShieldCurrent` Shield)
  (set `self.ShieldActive` true)
  (`KismetSystemLibrary.Delay` 10.0)
  (set `self.ShieldActive` false))

(event `/Game/Hordible/Placeables/Pickups/BPI_PickUp.PickupInvisibility`
  ;[1 1 1] When Invisible Active Set material to Invisible Material
  (`PrimitiveComponent.SetMaterial` (`self.Shield`) 0 "/Game/Hordible/MaterialLibrary/MI_Weapons.MI_Weapons")
  (`KismetSystemLibrary.Delay` 5.0)
  (`PrimitiveComponent.SetMaterial` (`self.Shield`) 0 "/Game/Hordible/MaterialLibrary/M_Weapons.M_Weapons"))

(event `/Game/Hordible/Core/Weapons/BPI_Recoil.Pistol_Recoil`
  ;[1 0 0.009453 1 17] Recoil Interface Event For Pistol
  (`self.AddControllerPitchInput` (`KismetMathLibrary.RandomFloatInRange` -0.8 -1.0))
  (`self.AddControllerYawInput` (`KismetMathLibrary.RandomFloatInRange` -0.4 -0.8)))

(event `/Game/Hordible/Core/Weapons/BPI_Recoil.Rifle_Recoil`
  ;[1 0 0.009772] Recoil Interface Event For Rifle
  (`self.AddControllerPitchInput` (`KismetMathLibrary.RandomFloatInRange` -0.2 -0.5))
  (`self.AddControllerYawInput` (`KismetMathLibrary.RandomFloatInRange` -0.2 -0.4)))

(event `/Game/Hordible/Core/Weapons/BPI_Recoil.Shotgun_Recoil`
  ;[1 0 0 1 17] Recoil Interface Event For Shotgun
  (`self.AddControllerPitchInput` (`KismetMathLibrary.RandomFloatInRange` -0.4 -0.8))
  (`self.AddControllerYawInput` (`KismetMathLibrary.RandomFloatInRange` -0.5 0.4)))

(event `/Game/Hordible/Core/Weapons/BPI_Recoil.Grenade Launcher_Recoil`
  ;[1 0 0] Recoil Interface Event For Grenade Launcher
  (`self.AddControllerPitchInput` (`KismetMathLibrary.RandomFloatInRange` -1.5 -2.5))
  (`self.AddControllerYawInput` (`KismetMathLibrary.RandomFloatInRange` -1.0 -2.0)))

(event `/Game/Hordible/Core/Weapons/BPI_Recoil.Crossbow_Recoil`
  ;[1 0 0] Recoil Interface Event For Crossbow
  (`self.AddControllerPitchInput` (`KismetMathLibrary.RandomFloatInRange` -0.5 -1.5))
  (`self.AddControllerYawInput` (`KismetMathLibrary.RandomFloatInRange` -0.5 -1.0)))

(fn `TakeDamage`
  (params (damage :type "Float (double-precision)"))
  (if (`self.Damage Player`)
    (if (`self.ShieldActive`)
      (bind _output_get (set `self.ShieldCurrent` (- (`self.ShieldCurrent`) damage)))
      (`self.EHealthUpdated` damage)
      (if (<= _output_get 0.0)
        (set `self.ShieldActive` false))
      (else
        (bind _output_get_2 (set `self.HealthCurrent` (- (`self.HealthCurrent`) damage)))
        (`self.EHealthUpdated` damage)
        (if (not (`self.EffectActive`))
          (`self.Damage Effect`))
        (if (<= _output_get_2 0.0)
          (`self.EPlayerDeath`)
          (`self.K2_DestroyActor`))))
    (else
      (bind _output_get_3 (set `self.HealthCurrent` (+ (`self.HealthCurrent`) damage)))
      (`KismetSystemLibrary.PrintString` (`KismetStringLibrary.Conv_DoubleToString` _output_get_3))
      (if (> (`self.HealthCurrent`) 51.0)
        (`/Game/Hordible/Core/UI/WBP_BloodSplatter.Remove` (`self.DamageUI`))
        (set `self.EffectActive` false)))))

(fn `UserConstructionScript`
  (bind _charactermovement (`self.CharacterMovement`))
  (set `CharacterMovementComponent.JumpZVelocity` (`self.JumpHeight`) _charactermovement)
  (set `CharacterMovementComponent.MaxWalkSpeed` (`self.WalkSpeed`) _charactermovement)
  (set `self.HealthCurrent` (`self.HealthMax`)))
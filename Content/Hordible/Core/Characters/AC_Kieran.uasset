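; AC_Kieran is a component holding the shield melee attack, apparently for the Kieran character in Hordible.
; Init stores a camera reference; MeleeAttack box-traces from it along player 0's control rotation, with debug drawing.
; Each hit actor's name is printed and it receives PlayerDamage through a DamageEnemy interface message.
; Hit Characters get a strong impulse opposite their own forward vector, not away from the attacker.
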(event `Init`
  (params (Camera :type "CameraComponent Object Reference"))
  (set `self.Camera` Camera))

(event `Melee Attack`
  (bind _radius (`self.Radius`))
  (bind _returnvalue (`SceneComponent.K2_GetComponentLocation` (`self.Camera`)))
  ;[1 1 1] Shield Attack
  (bind _outhits (`KismetSystemLibrary.BoxTraceMulti` :`Start` _returnvalue :`End` (+ _returnvalue (* (`KismetMathLibrary.GetForwardVector` (`Controller.GetControlRotation` (`GameplayStatics.GetPlayerController` 0))) (`self.meleeRange`))) :`HalfSize` (`KismetMathLibrary.MakeVector` _radius _radius _radius) :`TraceChannel` "TraceTypeQuery3" :`DrawDebugType` "ForDuration"))
  (for _array_element _outhits
    (bind (_bblockinghit _binitialoverlap _time _distance _location _impactpoint _normal _impactnormal _physmat _hitactor) (`GameplayStatics.BreakHitResult` _array_element))
    (`KismetSystemLibrary.PrintString` (`KismetSystemLibrary.GetDisplayName` _hitactor))
    (message `/Game/Hordible/Core/AI/BPI_DamageEnemy.DamageEnemy` _hitactor (`self.playerDamage`))
    (bind _ascharacter (cast `Character` _hitactor))
    (`CharacterMovementComponent.AddImpulse` (`Character.CharacterMovement` _ascharacter) (* (`Actor.GetActorForwardVector` _hitactor) -500000.0) false)))
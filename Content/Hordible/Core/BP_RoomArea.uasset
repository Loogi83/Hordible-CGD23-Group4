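; BP_RoomArea is a room trigger volume that selects which enemy spawner is active based on the room the player enters.
; When a BP_Character overlaps its Box, it deactivates every BP_EnemySpawner in the level, then activates its referenced SpawnerRef if valid.
; It also caches the GM_Wave game mode on BeginPlay, though the graphs shown never use it.
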(event `self.ReceiveBeginPlay`
  (set `self.As GM Wave` (cast `/Game/Hordible/Core/GameModes/GM_Wave` (`GameplayStatics.GetGameMode`) :!pure true)))

(event `self.Box.OnComponentBeginOverlap`
  (params (OverlappedComponent :type "PrimitiveComponent Object Reference") (OtherActor :type "Actor Object Reference") (OtherComp :type "PrimitiveComponent Object Reference") (OtherBodyIndex :type Integer) (bFromSweep :type Boolean) (SweepResult :type "HitResult Structure (by ref)"))
  (bind _spawnerref (`self.SpawnerRef`))
  (cast `/Game/Hordible/Core/Characters/BP_Character` OtherActor)
  (bind _outactors (`GameplayStatics.GetAllActorsOfClass` "/Game/Hordible/Core/Enemies/BP_EnemySpawner.BP_EnemySpawner_C"))
  (for _array_element _outactors
    (set `/Game/Hordible/Core/Enemies/BP_EnemySpawner.bActive` false _array_element))
  (`/Engine/EditorBlueprintResources/StandardMacros.IsValid` _spawnerref
    (:`Is Valid`
      (set `/Game/Hordible/Core/Enemies/BP_EnemySpawner.bActive` true _spawnerref))))

(fn `UserConstructionScript`)
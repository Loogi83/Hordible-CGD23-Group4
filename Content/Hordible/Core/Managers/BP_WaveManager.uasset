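; BP_WaveManager runs the enemy wave loop, starting the first wave when the game state changes to Ingame.
; A small state machine moves between Prep, InProgress and EndWave, with a short delay before the next Prep.
; Each wave's row in the WavePlan data table maps enemy types to quantities, which BP_EnemySpawner spawns.
; EnemyKilled decrements the active count and ends the wave when none remain.
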(event `self.ReceiveBeginPlay`
  (bind _returnvalue (`GameplayStatics.GetActorOfClass` "/Game/Hordible/Core/Enemies/BP_EnemySpawner.BP_EnemySpawner_C"))
  (`/Engine/EditorBlueprintResources/StandardMacros.IsValid` _returnvalue
    (:`Is Valid`
      (bind _output_get (set `self.SpawnerRef` _returnvalue))
      (`/Game/Hordible/Core/Enemies/BP_EnemySpawner.Init` _output_get self))))

(event `/Game/Hordible/Core/GameModes/BPI_GameState.I_GameStateChanged`
  (params (newGameState :type "/Game/Hordible/Core/GameModes/E_GameState Enum" :default "NewEnumerator0"))
  (switch `/Game/Hordible/Core/GameModes/E_GameState` newGameState
    (:`NewEnumerator2`
      (`self.ChangeWaveState` "NewEnumerator0"))))

(event `Prep Wave`
  (`self.StartWave` (`self.WaveNumber`))
  (`self.ChangeWaveState` "NewEnumerator1"))

(event `End Wave`
  (`KismetSystemLibrary.PrintString` "Wave Ended" true true (struct :`R` 1.0 :`G` 0.019788 :`A` 1.0) 10.0)
  (`/Engine/EditorBlueprintResources/StandardMacros.IncrementInt` (`self.WaveNumber`)
    (:`  `
      (`KismetSystemLibrary.Delay` 5.0)
      (`self.ChangeWaveState` "NewEnumerator0"))))

(event `Enemy Killed`
  (bind _active (`self.Active`))
  (`/Engine/EditorBlueprintResources/StandardMacros.DecrementInt` _active
    (:`  `
      (if (<= _active 0)
        (`self.ChangeWaveState` "NewEnumerator2")))))

(fn `ChangeWaveState`
  (params (NewWaveState :type "/Game/Hordible/Core/Managers/EWaveState Enum" :default "NewEnumerator0"))
  (bind _output_get (set `self.CurrentWaveState` NewWaveState))
  (switch `/Game/Hordible/Core/Managers/EWaveState` _output_get
    (:`NewEnumerator0`
      (`self.Prep Wave`))
    (:`NewEnumerator2`
      (`self.End Wave`))))

(fn `StartWave`
  (params (WaveNumber :type Integer))
  (bind _returnvalue (`|GetDataTableRow` (`self.WavePlan`) (`KismetStringLibrary.Conv_StringToName` (`KismetStringLibrary.Concat_StrStr` (`KismetStringLibrary.Conv_NameToString` "Wave") (`KismetStringLibrary.Conv_IntToString` WaveNumber))))
    (:`then`
      (bind _enemies (break `/Game/Hordible/Core/Managers/SWaveStats` _returnvalue))
      (bind _keys (`BlueprintMapLibrary.Map_Keys` _enemies))
      (for _array_element _keys
        (`/Game/Hordible/Core/Enemies/BP_EnemySpawner.SpawnEnemies` (`self.SpawnerRef`) _array_element (`BlueprintMapLibrary.Map_Find` _enemies _array_element))))))

(fn `UserConstructionScript`)
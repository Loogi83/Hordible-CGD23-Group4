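; Base enemy Blueprint for Hordible, handling stats, damage, death and melee-range detection.
; The construction script applies the Stats struct to health, walk speed and melee sphere radius, whose overlaps with BP_Character toggle CanMelee.
; Damage fires the EnemyDamaged dispatcher, bound in Init, and reduces health, with death firing EnemyKilled before destroying the actor.
; A separate event spawns damage-number popups, and Tick draws current health as debug text.
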(event `Init`
  (params (Manager :type "/Game/Hordible/Core/Managers/BP_WaveManager Object Reference"))
  (set `self.Manager` Manager)
  (add `self.EEnemyDamaged` (`|CreateDelegate` :!event `SpawnDamagePopup`)))

(event `/Game/Hordible/Core/AI/BPI_DamageEnemy.DamageEnemy`
  (params (DamageToDeal :type "Float (double-precision)"))
  (`self.TakeDamage` DamageToDeal))

(event `self.ReceiveTick`
  (params (DeltaSeconds :type "Float (single-precision)"))
  (`KismetSystemLibrary.DrawDebugString` (0.0 0.0 100.0) (`KismetStringLibrary.Conv_DoubleToString` (`.CurrentHealth_4_84644DB54A34569CA27C329BDE205092` (break `/Game/Hordible/Core/Enemies/S_EnemyStats` (`self.Stats`)))) self (struct :`A` 1.0)))

(event `self.Collision_MeleeRange.OnComponentBeginOverlap`
  (params (OverlappedComponent :type "PrimitiveComponent Object Reference") (OtherActor :type "Actor Object Reference") (OtherComp :type "PrimitiveComponent Object Reference") (OtherBodyIndex :type Integer) (bFromSweep :type Boolean) (SweepResult :type "HitResult Structure (by ref)"))
  (cast `/Game/Hordible/Core/Characters/BP_Character` OtherActor)
  (set `self.CanMelee` true))

(event `self.Collision_MeleeRange.OnComponentEndOverlap`
  (params (OverlappedComponent :type "PrimitiveComponent Object Reference") (OtherActor :type "Actor Object Reference") (OtherComp :type "PrimitiveComponent Object Reference") (OtherBodyIndex :type Integer))
  (cast `/Game/Hordible/Core/Characters/BP_Character` OtherActor)
  (set `self.CanMelee` false))

(event `SpawnDamagePopup` :!signature `self.EEnemyDamaged`
  (params (Amount :type "Float (double-precision)"))
  ;[1 1 1] Cheeky bit of UI for damage stats
  (`|SpawnActorFromClass` "/Game/Hordible/Core/UI/PopupTextWidgets/BP_TextPopup.BP_TextPopup_C" (`KismetMathLibrary.MakeTransform` (`self.K2_GetActorLocation`)) "Undefined" "OverrideRootScale" null (`KismetStringLibrary.Conv_DoubleToString` Amount) (struct :`R` 1.0 :`G` 0.012647 :`A` 1.0) null)
  (`KismetSystemLibrary.PrintString` "Damaging Enemy"))

(fn `Death`
  (`KismetSystemLibrary.PrintString` (`KismetStringLibrary.Concat_StrStr` (`KismetSystemLibrary.GetDisplayName` self) " has died!"))
  (`self.EEnemyKilled` self)
  (`self.K2_DestroyActor`))

(fn `TakeDamage`
  (params (DamageDealt :type "Float (double-precision)"))
  (bind (_movementspeed _currenthealth) (break `/Game/Hordible/Core/Enemies/S_EnemyStats` (`self.Stats`)))
  (`self.EEnemyDamaged` DamageDealt)
  (setmembers `/Game/Hordible/Core/Enemies/S_EnemyStats` :`StructRef` (`self.Stats`) :`CurrentHealth` (- _currenthealth DamageDealt))
  (if (<= _currenthealth 0.0)
    (`self.Death`)))

(fn `UserConstructionScript`
  (bind _stats (`self.Stats`))
  (bind ((`MovementSpeed_2_28FA2C6348DBB2A1392799B2F3D03407` _movementspeed) (`MaxHealth_6_D9738A614FE71AD569592B8B8F0B25C8` _maxhealth) (`Range_10_B15BB72946686B2C2C713B9A915B6090` _range)) (break `/Game/Hordible/Core/Enemies/S_EnemyStats` _stats))
  ;[1 1 1] Sets current health to max (saves manually changing both stats)
  (setmembers `/Game/Hordible/Core/Enemies/S_EnemyStats` :`StructRef` _stats :`CurrentHealth` _maxhealth)
  ;[1 1 1] Sets character movement speed as struct variable
  (set `CharacterMovementComponent.MaxWalkSpeed` _movementspeed (`self.CharacterMovement`))
  ;[1 1 1] Sets melee collision radius to stats range
  (`SphereComponent.SetSphereRadius` (`self.Collision_MeleeRange`) _range true))
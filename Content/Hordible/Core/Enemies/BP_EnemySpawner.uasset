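; BP_EnemySpawner is a spawn point actor that creates enemies of a requested class for its manager.
; Init stores the manager reference, and SpawnEnemies spawns one enemy, adjusting for collisions, then registers it through the manager's AddEnemy.
; Spawn locations are random navmesh-reachable points within SpawnRadius, lifted slightly above the ground.
; The construction script sizes a sphere component to show that radius.
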(event `Init`
  (params (Manager :type "/Game/Hordible/Core/Managers/BP_WaveManager Object Reference"))
  ;[1 1 1] Init
  (set `self.Manager` Manager))

(event `SpawnEnemies`
  (params (EnemyType :type "/Game/Hordible/Core/Enemies/BP_BaseEnemy Class Reference"))
  ;[0.1473 1 0] Spawn Enemies
  (bind _spawnlocation (`self.GetSpawnLocation`))
  (bind _returnvalue (`|SpawnActorFromClass` EnemyType (`KismetMathLibrary.MakeTransform` _spawnlocation) "AdjustIfPossibleButAlwaysSpawn" "OverrideRootScale" null null))
  (`/Game/Hordible/Core/Managers/BP_WaveManager.AddEnemy` (`self.Manager`) _returnvalue))

(fn `GetSpawnLocation`
  (returns (SpawnLocation :type "Vector Structure"))
  (return (+ (`NavigationSystemV1.K2_GetRandomReachablePointInRadius` (`self.K2_GetActorLocation`) (`self.SpawnRadius`) null null) (0.0 0.0 20.0))))

(fn `UserConstructionScript`
  (`SphereComponent.SetSphereRadius` (`self.Sphere`) (`self.SpawnRadius`) true))
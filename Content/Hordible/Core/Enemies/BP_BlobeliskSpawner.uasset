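; BP_BlobeliskSpawner is a spawn point that creates a BP_Blobelisk enemy on every even-numbered wave.
; When the game state changes to Ingame, it finds and stores the BP_WaveManager.
; Its NewWave event spawns the Blobelisk at the spawner's transform, adjusting for collision but always spawning, then registers it with the manager through AddBlobelisk.
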(event `/Game/Hordible/Core/Managers/BPI_NewWave.NewWave`
  (params (WaveNumber :type Integer))
  (if (== (mod WaveNumber 2) 0)
    (`self.SpawnEnemy`)))

(event `/Game/Hordible/Core/GameModes/BPI_GameState.I_GameStateChanged`
  (params (newGameState :type "/Game/Hordible/Core/GameModes/E_GameState Enum" :default "NewEnumerator0"))
  (switch `/Game/Hordible/Core/GameModes/E_GameState` newGameState
    (:`NewEnumerator2`
      (bind _returnvalue (`GameplayStatics.GetActorOfClass` "/Game/Hordible/Core/Managers/BP_WaveManager.BP_WaveManager_C"))
      (set `self.Manager` _returnvalue))))

(fn `SpawnEnemy`
  (bind _returnvalue (`|SpawnActorFromClass` "/Game/Hordible/Enemies/Enemies/Blobelisk/BP_Blobelisk.BP_Blobelisk_C" (`self.GetTransform`) "AdjustIfPossibleButAlwaysSpawn" "OverrideRootScale" null null))
  (`/Game/Hordible/Core/Managers/BP_WaveManager.Add Blobelisk` (`self.Manager`) _returnvalue))

(fn `UserConstructionScript`)
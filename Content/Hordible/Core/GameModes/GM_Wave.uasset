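; GM_Wave is the wave-mode game mode, running a match through Setup, Pregame, InGame and PostGame states via ChangeGameState.
; Setup binds to player death, then Pregame spawns and initializes BP_WaveManager and creates the in-game widget.
; InGame shows that widget and listens for the manager's ECanEnd event.
; CanEnd advances the state, and PostGame returns to the main menu after a short delay.
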(event `self.ReceiveBeginPlay`
  ;[1 1 1] Init
  (`KismetSystemLibrary.PrintString` "GM_Wave Active")
  (`parent.ReceiveBeginPlay`))

(event `self.Setup`
  ;[0 1 0.04752] Game States
  (bind _asbp_character (cast `/Game/Hordible/Core/Characters/BP_Character` (`GameplayStatics.GetPlayerCharacter` 0)))
  (add `/Game/Hordible/Core/Characters/BP_Character.EPlayerDeath` _asbp_character (`|CreateDelegate` :!event `Can End`))
  (`self.changeGameState` "NewEnumerator1"))

(event `self.Pregame`
  ;[0 1 0.04752] Game States
  (bind _returnvalue (`|SpawnActorFromClass` "/Game/Hordible/Core/Managers/BP_WaveManager.BP_WaveManager_C" (`KismetMathLibrary.MakeTransform` (0.0 0.0 0.0)) "Undefined" "OverrideRootScale" null -1 null))
  (bind _output_get (set `self.Manager` _returnvalue))
  (`/Game/Hordible/Core/Managers/BP_WaveManager.Init` _output_get)
  (bind _returnvalue_2 (`|CreateWidget` "/Game/Hordible/Core/UI/WBP_Ingame.WBP_Ingame_C"))
  (set `self.UI` _returnvalue_2)
  (`self.changeGameState` "NewEnumerator2"))

(event `self.InGame`
  ;[0 1 0.04752] Game States
  (`UserWidget.AddToViewport` (`self.UI`) 0)
  (add `/Game/Hordible/Core/Managers/BP_WaveManager.ECanEnd` (`self.Manager`) (`|CreateDelegate` :!event `Can End`)))

(event `self.PostGame`
  ;[0 1 0.04752] Game States
  (`KismetSystemLibrary.PrintString` "Game End")
  (`KismetSystemLibrary.Delay` 2.0)
  (`GameplayStatics.OpenLevel` "Level_MainMenu"))

(event `Can End`
  (`self.changeGameState` "NewEnumerator3"))

(fn `UserConstructionScript`
  (`parent.UserConstructionScript`))
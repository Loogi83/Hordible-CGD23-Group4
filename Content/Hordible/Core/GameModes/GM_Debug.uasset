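; GM_Debug is a game mode for Hordible that holds the current game state and enters Setup on BeginPlay.
; ChangeGameState stores and prints the new state, then broadcasts it through the BPI_GameState interface to every implementing actor and widget, including nested widgets.
; Its own IGameStateChanged event routes Setup, Pregame, Ingame and Postgame to per-state events, all currently empty stubs.
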(event `self.ReceiveBeginPlay`
  ;[1 1 1] Init
  (`self.changeGameState` "NewEnumerator0"))

(event `Setup`
  ;[0 1 0.07538] Game States
)

(event `/Game/Hordible/Core/GameModes/BPI_GameState.I_GameStateChanged`
  (params (newGameState :type "/Game/Hordible/Core/GameModes/E_GameState Enum" :default "NewEnumerator0"))
  ;[0 0.5462 1] Game State Changed
  (switch `/Game/Hordible/Core/GameModes/E_GameState` newGameState
    (:`NewEnumerator0`
      (`self.Setup`))
    (:`NewEnumerator1`
      (`self.Pregame`))
    (:`NewEnumerator2`
      (`self.InGame`))
    (:`NewEnumerator3`
      (`self.PostGame`))))

(event `Pregame`
  ;[0 1 0.07538] Game States
)

(event `InGame`
  ;[0 1 0.07538] Game States
)

(event `PostGame`
  ;[0 1 0.07538] Game States
)

(fn `changeGameState`
  (params (newGameState :type "/Game/Hordible/Core/GameModes/E_GameState Enum" :default "NewEnumerator0"))
  (set `self.currentGameState` newGameState)
  (`KismetSystemLibrary.PrintString` (`KismetStringLibrary.Concat_StrStr` "Game State changed to: " (`|GetEnumeratorNameAsString` newGameState)))
  (bind _outactors (`GameplayStatics.GetAllActorsWithInterface` "/Game/Hordible/Core/GameModes/BPI_GameState.BPI_GameState_C"))
  (for _array_element _outactors
    (message `/Game/Hordible/Core/GameModes/BPI_GameState.I_GameStateChanged` _array_element (`local.newGameState`)))
  (bind _foundwidgets (`WidgetBlueprintLibrary.GetAllWidgetsWithInterface` "/Game/Hordible/Core/GameModes/BPI_GameState.BPI_GameState_C"))
  (for _array_element_2 _foundwidgets
    (message `/Game/Hordible/Core/GameModes/BPI_GameState.I_GameStateChanged` _array_element_2 (`local.newGameState`))))

(fn `UserConstructionScript`)
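; BP_Door is a door actor that swings open when a specified wave number is reached.
; It snaps to its start rotation on BeginPlay, and its NewWave event calls OpenDoor when the wave matches TargetWave.
; OpenDoor plays a timeline that lerps the scene root's relative rotation from start to target.
; The construction script applies the configurable DoorMesh to the Door component.
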(event `self.ReceiveBeginPlay`
  (`self.K2_SetActorRotation` (`self.StartRotation`)))

(event `/Game/Hordible/Core/Managers/BPI_NewWave.NewWave`
  (params (WaveNumber :type Integer))
  (if (== WaveNumber (`self.TargetWave`))
    (`self.OpenDoor`)))

(event `OpenDoor`
  (bind (_direction _alpha) (`Timeline|OpenTimeline` :!via `PlayFromStart`)
    (:`Update`
      (`SceneComponent.K2_SetRelativeRotation` (`self.DefaultSceneRoot`) (`KismetMathLibrary.RLerp` (`self.StartRotation`) (`self.TargetRotation`) _alpha) false false))))

(fn `UserConstructionScript`
  (`StaticMeshComponent.SetStaticMesh` (`self.Door`) (`self.DoorMesh`)))
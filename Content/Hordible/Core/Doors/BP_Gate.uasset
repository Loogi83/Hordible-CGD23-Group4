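; BP_Gate is a gate that slides open when a specific wave number begins.
; Its NewWave event compares the incoming number to TargetWave and calls OpenDoor on a match.
; OpenDoor plays a timeline that lerps the Door mesh's relative location from the origin to TargetLocation, without sweep.
; The construction script applies the DoorMesh variable to the Door component.
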(event `/Game/Hordible/Core/Managers/BPI_NewWave.NewWave`
  (params (WaveNumber :type Integer))
  (if (== WaveNumber (`self.TargetWave`))
    (`self.OpenDoor`)))

(event `OpenDoor`
  (bind (_direction _alpha) (`Timeline|OpenTimeline` :!via `PlayFromStart`)
    (:`Update`
      (`SceneComponent.K2_SetRelativeLocation` (`self.Door`) (`KismetMathLibrary.VLerp` (0.0 0.0 0.0) (`self.TargetLocation`) _alpha) false false))))

(fn `UserConstructionScript`
  (`StaticMeshComponent.SetStaticMesh` (`self.Door`) (`self.DoorMesh`)))
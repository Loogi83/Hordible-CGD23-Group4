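; BP_BlobcadeAreaSpawner is a trigger actor that spawns a BP_Blobcade when the player character leaves its area.
; When a BP_Character ends overlap with its Box and CanSpawn is true, SpawnBlobcade creates the Blobcade at the spawner's own location and rotation.
; It then clears CanSpawn, and nothing in this graph sets it back, so it fires only once.
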(event `self.Box.OnComponentEndOverlap`
  (params (OverlappedComponent :type "PrimitiveComponent Object Reference") (OtherActor :type "Actor Object Reference") (OtherComp :type "PrimitiveComponent Object Reference") (OtherBodyIndex :type Integer))
  (if (`self.bCanSpawn`)
    (cast `/Game/Hordible/Core/Characters/BP_Character` OtherActor)
    (`self.SpawnBlobcade`)))

(fn `SpawnBlobcade`
  (`|SpawnActorFromClass` "/Game/Hordible/Enemies/Enemies/Blobcade/BP_Blobcade.BP_Blobcade_C" (`KismetMathLibrary.MakeTransform` (`self.K2_GetActorLocation`) (`self.K2_GetActorRotation`)) "Undefined" "OverrideRootScale" null null)
  (set `self.bCanSpawn` false))

(fn `UserConstructionScript`
  (`parent.UserConstructionScript`))
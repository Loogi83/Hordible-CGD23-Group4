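; BP_InvisibilityPickup is a pickup that triggers an invisibility effect when a BP_Character overlaps its sphere.
; The overlap sends PickupInvisibilityMessage to the character and its "Gun"-tagged child actors, then calls AddACInvisible on every BP_BaseEnemy in the level.
; A separate Pickup function disables sphere collision and hides the actor, but the overlap does not call it.
; An unconnected chain that briefly freezes enemy movement never runs.
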(event `self.Sphere.OnComponentBeginOverlap`
  (params (OverlappedComponent :type "PrimitiveComponent Object Reference") (OtherActor :type "Actor Object Reference") (OtherComp :type "PrimitiveComponent Object Reference") (OtherBodyIndex :type Integer) (bFromSweep :type Boolean) (SweepResult :type "HitResult Structure (by ref)"))
  ;[0.6146 0.6146 0.6146] Activate Invisibility Pickup Interface and add Actor Component to Active Enemies on Collision
  (bind _asbp_character (cast `/Game/Hordible/Core/Characters/BP_Character` OtherActor))
  (message `/Game/Hordible/Placeables/Pickups/BPI_PickUp.PickupInvisibility` _asbp_character)
  (for _array_element (`self.GetComponentsByTag` _asbp_character "/Script/Engine.ChildActorComponent" "Gun")
    (message `/Game/Hordible/Placeables/Pickups/BPI_PickUp.PickupInvisibility` (`ChildActorComponent.ChildActor` (cast `ChildActorComponent` _array_element :!pure true))))
  (bind _outactors (`GameplayStatics.GetAllActorsOfClass` "/Game/Hordible/Core/Enemies/BP_BaseEnemy.BP_BaseEnemy_C"))
  (for _array_element_2 _outactors
    (`AddComponent|NODE_AddAC_Invisible-0` :`self` _array_element_2)))

(fn `Pickup`
  (`PrimitiveComponent.SetCollisionEnabled` (`self.Sphere`) "NoCollision")
  (`self.SetActorHiddenInGame` true))

(fn `UserConstructionScript`
  (`parent.UserConstructionScript`))
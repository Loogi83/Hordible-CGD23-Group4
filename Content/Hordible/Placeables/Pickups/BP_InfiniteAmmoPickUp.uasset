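; BP_InfiniteAmmoPickUp is a pickup that grants infinite ammo to the player character's guns.
; On sphere overlap with BP_Character, it plays the Bottomless Clip sound cue and finds every ChildActorComponent tagged "Gun".
; It sends the InfiniteAmmoMessage to each gun's child actor to switch infinite ammo on.
; Its Pickup function and construction script only call the parent versions, and nothing here turns the effect off.
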(event `self.Sphere.OnComponentBeginOverlap`
  (params (OverlappedComponent :type "PrimitiveComponent Object Reference") (OtherActor :type "Actor Object Reference") (OtherComp :type "PrimitiveComponent Object Reference") (OtherBodyIndex :type Integer) (bFromSweep :type Boolean) (SweepResult :type "HitResult Structure (by ref)"))
  ;[0.6492 1 0 1 17] Activate Infinite Ammo for Each Weapon On Collision
  (bind _asbp_character (cast `/Game/Hordible/Core/Characters/BP_Character` OtherActor))
  (`GameplayStatics.PlaySound2D` "/Game/Hordible/Core/Sounds/Nathan/Bottomless_Clip_mock-up_Cue.Bottomless_Clip_mock-up_Cue" 1.0 1.0 0.0 null null)
  (for _array_element (`self.GetComponentsByTag` _asbp_character "/Script/Engine.ChildActorComponent" "Gun")
    (message `/Game/Hordible/Core/Weapons/BPI_Weapons.InfiniteAmmo` (`ChildActorComponent.ChildActor` (cast `ChildActorComponent` _array_element :!pure true)) true)))

(fn `Pickup`
  (`parent.Pickup`))

(fn `UserConstructionScript`
  (`parent.UserConstructionScript`))
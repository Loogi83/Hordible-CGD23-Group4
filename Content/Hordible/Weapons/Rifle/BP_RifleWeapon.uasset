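; Rifle weapon Blueprint for the player, handling automatic fire, ammo, reloading and timed pickup effects.
; Attack starts a looping timer that fires cone-spread line traces against Pawns, sending damage to hit actors and recoil to BP_Character.
; Timelines animate recoil and reload dip; running out or manual reload shows a reload widget, then refills ammo.
; Pickup events temporarily stop ammo consumption or swap the mesh material for invisibility.
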(event `/Game/Hordible/Core/Weapons/BPI_Weapons.InfiniteAmmo`
  (params (Active :type Boolean))
  ;[1 1 1] When Infinite Ammo Active set boolean to true and then to false after 5 seconds
  (set `self.Active` Active)
  (`KismetSystemLibrary.Delay` 5.0)
  (set `self.Active` false))

(event `/Game/Hordible/Placeables/Pickups/BPI_PickUp.PickupInvisibility`
  ;[1 1 1] When Invisible Active Set material to Invisible Material
  (`PrimitiveComponent.SetMaterial` (`self.Cube`) 0 "/Game/Hordible/MaterialLibrary/MI_Weapons.MI_Weapons")
  (`KismetSystemLibrary.Delay` 5.0)
  (`PrimitiveComponent.SetMaterial` (`self.Cube`) 0 "/Game/Hordible/MaterialLibrary/M_Weapons.M_Weapons"))

(event `self.ReceiveBeginPlay`
  (bind _cube (`self.Cube`))
  ;[1 1 1] Set Weapon Location and Rotation
  (set `self.Start Location` (`SceneComponent.RelativeLocation` _cube))
  (set `self.Start Rotation` (`SceneComponent.RelativeRotation` _cube)))

(event `RunOut`
  ;[1 0.2057 0] Assualt Rifle Basic Firing Function with Fire rate, Damage, Fire Spread, and Range Variables
  (`ActorComponent.Activate` (`self.Niagara`) true :!label _label)
  (`self.Reload Icon Anim`)
  (bind (_direction _reloadgun) (`Timeline|ReloadingRifle` :!via `PlayFromStart`)
    (:`Update`
      (`SceneComponent.K2_SetRelativeLocation` (`self.Cube`) (`KismetMathLibrary.VLerp` (`self.Start Location`) (- (`self.Start Location`) (`KismetMathLibrary.MakeVector` 0.0 0.0 (`self.Reload Target Location`))) _reloadgun) false false))
    (:`Finished`
      (set `self.Current Ammo` (`self.MaxAmmo`))
      (set `self.CanFire` true))))

(event `self.Manual Reload`
  ;[1 0.2057 0] Assualt Rifle Basic Firing Function with Fire rate, Damage, Fire Spread, and Range Variables
  (set `self.CanFire` false)
  (goto _label))

(event `self.Attack`
  ;[1 0.2057 0] Assualt Rifle Basic Firing Function with Fire rate, Damage, Fire Spread, and Range Variables
  (if (`self.CanFire`)
    (set `self.CanFire` false)
    (if (< (`self.Current Ammo`) 0)
      (goto _label)
      (else
        (`self.Fire`)
        (bind _returnvalue (`KismetSystemLibrary.K2_SetTimerDelegate` (delegate `self.Fire`) (`self.RifleFireRate`) true))
        (set `self.Gun Timer Ref` _returnvalue)))))

(event `self.Fire`
  (bind _start_location (`self.Start Location`))
  (bind _start_rotation (`self.Start Rotation`))
  (bind _current_ammo (`self.Current Ammo`))
  (bind _returnvalue (`SceneComponent.K2_GetComponentLocation` (`self.Arrow`)))
  (bind _returnvalue_2 (`Controller.GetControlRotation` (`GameplayStatics.GetPlayerController` 0)))
  ;[1 0.2057 0] Assualt Rifle Basic Firing Function with Fire rate, Damage, Fire Spread, and Range Variables
  (if (< (`self.Current Ammo`) 0)
    (`KismetSystemLibrary.Delay` 0.2)
    (set `self.CanFire` false)
    (`KismetSystemLibrary.K2_ClearAndInvalidateTimerHandle` (`self.Gun Timer Ref`))
    (`self.RunOut`)
    (else
      (bind _outhit (`KismetSystemLibrary.LineTraceSingleForObjects` :`Start` _returnvalue :`End` (+ _returnvalue (* (`KismetMathLibrary.RandomUnitVectorInConeInDegrees` (`KismetMathLibrary.GetForwardVector` _returnvalue_2) (`self.Fire Spread`)) (`self.RifleRange`))) :`ObjectTypes` (`|MakeArray` "ObjectTypeQuery3" :!type "EObjectTypeQuery Enum") :`DrawTime` 0.1))
      (`NiagaraFunctionLibrary.SpawnSystemAtLocation` "/Game/Hordible/Core/Particles/NS_RifleFire.NS_RifleFire" _returnvalue _returnvalue_2)
      (bind _asbp_character (cast `/Game/Hordible/Core/Characters/BP_Character` (`GameplayStatics.GetPlayerCharacter` 0)))
      (message `/Game/Hordible/Core/Weapons/BPI_Recoil.Rifle_Recoil` _asbp_character)
      (if (not (`self.Active`))
        (`/Engine/EditorBlueprintResources/StandardMacros.DecrementInt` _current_ammo
          (:`  `
            (`KismetSystemLibrary.PrintString` (`KismetStringLibrary.Concat_StrStr` "Current Ammo = " (`KismetStringLibrary.Conv_IntToString` _current_ammo)) true true (struct :`R` 1.0 :`G` 0.473853 :`A` 1.0) 0.1))))
      ;;[1 0 0.08529] Added this so rifle can damage enemies - Kieran
      (message `/Game/Hordible/Core/AI/BPI_DamageEnemy.DamageEnemy` (`.HitActor` (`GameplayStatics.BreakHitResult` _outhit)) (`self.RifleDamage`))
      (`KismetSystemLibrary.K2_SetTimerDelegate` (delegate `Reload`) (`self.FireRate`))
      (bind (_direction _recoil) (`Timeline|Recoil` :!via `PlayFromStart`)
        (:`Update`
          (`SceneComponent.K2_SetRelativeLocationAndRotation` (`self.Cube`) (`KismetMathLibrary.VLerp` _start_location (+ _start_location (-10.0 20.0 15.0)) _recoil) (`KismetMathLibrary.RLerp` _start_rotation (`KismetMathLibrary.ComposeRotators` _start_rotation (struct :`Pitch` 7.0 :`Yaw` 7.0 :`Roll` 2.0)) _recoil true) false false))))))

(event `Reload`
  ;[1 0.2057 0] Assualt Rifle Basic Firing Function with Fire rate, Damage, Fire Spread, and Range Variables
  (set `self.CanFire` true))

(event `Reload Icon Anim`
  (bind _returnvalue (`|CreateWidget` "/Game/Hordible/Core/UI/WBP_ReloadIcon.WBP_ReloadIcon_C"))
  (`UserWidget.AddToViewport` _returnvalue 0))

(fn `UserConstructionScript`
  (`parent.UserConstructionScript`)
  (set `self.Current Ammo` (`self.MaxAmmo`)))
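; Actor component from the shotgun weapon that briefly stuns the BP_BaseEnemy it is attached to.
; On BeginPlay it spawns a stun Niagara effect at the enemy mesh, disables movement and shrinks the melee range sphere to zero.
; After a fixed two-second delay it restores NavWalking and a hardcoded melee radius, then destroys itself, so adding the component is what triggers the stun.
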(event `self.ReceiveBeginPlay`
  (bind _asbp_base_enemy (cast `/Game/Hordible/Core/Enemies/BP_BaseEnemy` (`self.GetOwner`)))
  (`NiagaraFunctionLibrary.SpawnSystemAtLocation` "/Game/Hordible/Core/Particles/NS_Stun.NS_Stun" (`SceneComponent.K2_GetComponentLocation` (`Character.Mesh` _asbp_base_enemy)))
  (bind _charactermovement (`Character.CharacterMovement` _asbp_base_enemy))
  (`CharacterMovementComponent.DisableMovement` _charactermovement)
  (bind _collision_meleerange (`/Game/Hordible/Core/Enemies/BP_BaseEnemy.Collision_MeleeRange` _asbp_base_enemy))
  (`SphereComponent.SetSphereRadius` _collision_meleerange 0.0 false)
  (`KismetSystemLibrary.Delay` 2.0)
  (`CharacterMovementComponent.SetMovementMode` _charactermovement "MOVE_NavWalking" 0)
  (`SphereComponent.SetSphereRadius` _collision_meleerange 103.08316 true)
  (`self.K2_DestroyComponent`))
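; Shotgun weapon for the player in Hordible, firing a spread of cone-randomised line traces that damage whatever they hit.
; Attack spends ammo and fires on a timer, auto-reloading when depleted, with timelines animating recoil and reload.
; An enemy hit also adds a stun when that ability is off its ten-second cooldown.
; Pickup events temporarily grant infinite ammo or swap the weapon material for invisibility.
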(event `/Game/Hordible/Placeables/Pickups/BPI_PickUp.PickupInvisibility`
  ;[1 1 1] When Invisible Active Set material to Invisible Material
  (`PrimitiveComponent.SetMaterial` (`self.Cube`) 0 "/Game/Hordible/MaterialLibrary/MI_Weapons.MI_Weapons")
  (`KismetSystemLibrary.Delay` 5.0)
  (`PrimitiveComponent.SetMaterial` (`self.Cube`) 0 "/Game/Hordible/MaterialLibrary/M_Weapons.M_Weapons"))

(event `self.ReceiveBeginPlay`
  (bind _cube (`self.Cube`))
  ;[0.4072 0.1144 0] Set Weapon Location and Rotation
  (set `self.Start Location` (`SceneComponent.RelativeLocation` _cube))
  (set `self.Start Rotation` (`SceneComponent.RelativeRotation` _cube)))

(event `/Game/Hordible/Core/Weapons/BPI_Weapons.InfiniteAmmo`
  (params (Active :type Boolean))
  ;[1 1 1] When Infinite Ammo Active set boolean to true and then to false after 5 seconds
  (set `self.Active` Active)
  (`KismetSystemLibrary.Delay` 5.0)
  (set `self.Active` false))

(event `self.Manual Reload`
  ;[1 0.279 0] Shotgun Line trace spread, damage and range
  (set `self.CanFire` false)
  (`ActorComponent.Activate` (`self.Niagara`) true :!label _label)
  (`self.Reload Icon Anim`)
  (bind (_direction _reloadgun) (`Timeline|ReloadingShotgun` :!via `PlayFromStart`)
    (:`Update`
      (`SceneComponent.K2_SetRelativeLocation` (`self.Cube`) (`KismetMathLibrary.VLerp` (`self.Start Location`) (- (`self.Start Location`) (`KismetMathLibrary.MakeVector` 0.0 0.0 (`self.ReloadTargetLocation`))) _reloadgun) false false))
    (:`Finished`
      (set `self.Current Ammo` (`self.maxAmmo`))
      (set `self.CanFire` true))))

(event `self.Attack`
  (bind _current_ammo (`self.Current Ammo`))
  ;[1 0.279 0] Shotgun Line trace spread, damage and range
  (if (`self.Active`)
    (`KismetSystemLibrary.K2_SetTimerDelegate` (delegate `self.Fire`) (`self.ShotgunFireRate`) :!label _label_2)
    (elif (`self.CanFire`)
      (set `self.CanFire` false)
      (`/Engine/EditorBlueprintResources/StandardMacros.DecrementInt` _current_ammo
        (:`  `
          (`KismetSystemLibrary.PrintString` (`KismetStringLibrary.Concat_StrStr` "Current Ammo = " (`KismetStringLibrary.Conv_IntToString` _current_ammo)) true true (struct :`R` 1.0 :`G` 0.591692 :`A` 1.0) 0.1)
          (if (< (`self.Current Ammo`) 0)
            (goto _label)
            (else
              (goto _label_2))))))))

(event `Reload`
  ;[1 0.279 0] Shotgun Line trace spread, damage and range
  (set `self.CanFire` true))

(event `self.Fire`
  (bind _start_location (`self.Start Location`))
  (bind _start_rotation (`self.Start Rotation`))
  (bind _returnvalue (`SceneComponent.K2_GetComponentLocation` (`self.Arrow`)))
  (bind _returnvalue_2 (`Controller.GetControlRotation` (`GameplayStatics.GetPlayerController` 0)))
  ;[1 0.279 0] Shotgun Line trace spread, damage and range
  (for _ (range 5)
    (bind _outhit (`KismetSystemLibrary.LineTraceSingle` :`Start` _returnvalue :`End` (+ _returnvalue (* (`KismetMathLibrary.RandomUnitVectorInConeInDegrees` (`KismetMathLibrary.GetForwardVector` _returnvalue_2) (`self.Fire Spread`)) (`self.ShotgunRange`))) :`TraceChannel` "TraceTypeQuery3" :`DrawTime` 0.1))
    (`NiagaraFunctionLibrary.SpawnSystemAtLocation` "/Game/Hordible/Core/Particles/NS_ShotgunFire.NS_ShotgunFire" _returnvalue _returnvalue_2)
    (bind _asbp_character (cast `/Game/Hordible/Core/Characters/BP_Character` (`GameplayStatics.GetPlayerCharacter` 0)))
    (message `/Game/Hordible/Core/Weapons/BPI_Recoil.Shotgun_Recoil` _asbp_character)
    (`|ExecutionSequence`
      (:`then_0`
        (bind (_bblockinghit _binitialoverlap _time _distance _location _impactpoint _normal _impactnormal _physmat _hitactor) (`GameplayStatics.BreakHitResult` _outhit))
        (cast `/Game/Hordible/Core/Enemies/BP_BaseEnemy` _hitactor
          (:`then`
            (if (`self.AbilityActive`)
              (message `/Game/Hordible/Core/AI/BPI_DamageEnemy.DamageEnemy` _hitactor (`self.ShotgunDamage`) :!label _label_3)
              (`KismetSystemLibrary.K2_SetTimerDelegate` (delegate `Reload`) 0.1)
              (else
                (set `self.AbilityActive` true)
                (message `/Game/Hordible/Core/AI/BPI_DamageEnemy.DamageEnemy` _hitactor (`self.ShotgunDamage`))
                (`KismetSystemLibrary.K2_SetTimerDelegate` (delegate `Reload`) 0.1)
                (bind _asbp_base_enemy (cast `/Game/Hordible/Core/Enemies/BP_BaseEnemy` _hitactor))
                (`AddComponent|NODE_AddAC_StunEnemies-0` :`self` _asbp_base_enemy)
                (`KismetSystemLibrary.K2_SetTimerDelegate` (delegate `AbilityReload`) 10.0))))
          (:`CastFailed`
            (goto _label_3))))
      (:`then_1`
        (bind (_direction _recoil) (`Timeline|Recoil` :!via `PlayFromStart`)
          (:`Update`
            (`SceneComponent.K2_SetRelativeLocationAndRotation` (`self.Cube`) (`KismetMathLibrary.VLerp` _start_location (+ _start_location (-10.0 20.0 15.0)) _recoil) (`KismetMathLibrary.RLerp` _start_rotation (`KismetMathLibrary.ComposeRotators` _start_rotation (struct :`Pitch` 10.0 :`Yaw` 14.0 :`Roll` 6.0)) _recoil true) false false)))))))

(event `AbilityReload`
  ;[1 0.279 0] Shotgun Line trace spread, damage and range
  (set `self.AbilityActive` false))

(event `Reload Icon Anim`
  ;[1 1 1] Reload Icon appearance and Animation
  (bind _returnvalue (`|CreateWidget` "/Game/Hordible/Core/UI/WBP_ReloadIcon.WBP_ReloadIcon_C"))
  (`UserWidget.AddToViewport` _returnvalue 0))

(fn `UserConstructionScript`
  (`parent.UserConstructionScript`)
  (set `self.Current Ammo` (`self.maxAmmo`)))
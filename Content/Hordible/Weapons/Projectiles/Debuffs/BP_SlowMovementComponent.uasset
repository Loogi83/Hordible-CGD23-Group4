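; BP_SlowMovementComponent is a projectile debuff component that slows a hit character.
; Init passes the hit actor to the parent implementation, and the Effect event casts it to BP_Character, caches its max walk speed and halves it.
; The DestroyComponent event writes the cached speed back to the character, undoing the slow.
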(event `Init`
  (params (HitActor :type "Actor Object Reference"))
  (`parent.Init` HitActor))

(event `self.Effect`
  (params (HitActor :type "Actor Object Reference"))
  ;[1 1 1] Halves max walk speed (stores ref to old max speed to revert back to)
  (bind _asbp_character (cast `/Game/Hordible/Core/Characters/BP_Character` HitActor))
  (bind _charactermovement (`Character.CharacterMovement` _asbp_character))
  (bind _maxwalkspeed (`CharacterMovementComponent.MaxWalkSpeed` _charactermovement))
  (set `self.oldMaxWalkSpeed` _maxwalkspeed)
  (set `CharacterMovementComponent.MaxWalkSpeed` (/ _maxwalkspeed 2.0) _charactermovement))

(event `self.DestroyComponent`
  ;[1 1 1] Reverts back to old max walk speed on destroy
  (set `CharacterMovementComponent.MaxWalkSpeed` (`self.oldMaxWalkSpeed`) (`Character.CharacterMovement` (stale `self.Effect` _asbp_character))))
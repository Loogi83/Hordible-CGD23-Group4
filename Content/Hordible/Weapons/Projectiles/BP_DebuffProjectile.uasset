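; BP_DebuffProjectile is a projectile Blueprint that puts a timed movement slow on the actor it hits.
; ApplyDebuff adds a BP_SlowMovementComponent to the hit actor at runtime and initializes it with that actor.
; It skips actors that already carry the component, so the slow neither stacks nor refreshes.
; Overlap handling passes straight to the parent class, and nothing in this graph calls ApplyDebuff.
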(event `self.ReceiveActorBeginOverlap`
  (params (OtherActor :type "Actor Object Reference"))
  (`parent.ReceiveActorBeginOverlap` OtherActor))

(event `/Game/Hordible/Weapons/Projectiles/BPI_AddDebuff.ApplyDebuff`
  (params (HitActor :type "Actor Object Reference"))
  ;[1 1 1] Applies DebuffComponent if Component is not currently on HitActor
  (if (not (`KismetSystemLibrary.IsValid` (`self.GetComponentByClass` HitActor "/Game/Hordible/Weapons/Projectiles/Debuffs/BP_SlowMovementComponent.BP_SlowMovementComponent_C")))
    (bind _returnvalue (`|AddComponentByClass` HitActor "/Game/Hordible/Weapons/Projectiles/Debuffs/BP_SlowMovementComponent.BP_SlowMovementComponent_C" 5.0))
    (`/Game/Hordible/Weapons/Projectiles/Debuffs/BP_BaseDebuffComponent.Init` _returnvalue HitActor)))

(fn `UserConstructionScript`
  (`parent.UserConstructionScript`))
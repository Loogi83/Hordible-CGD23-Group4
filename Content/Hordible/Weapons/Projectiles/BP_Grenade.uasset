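; BP_Grenade is a projectile that explodes on impact, dealing area damage and knocking enemies into the air.
; When its Sphere hits another actor, a multi-sphere object trace gathers WorldDynamic and Pawn objects within Radius, with debug drawing left on.
; Each hit receives a DamageEnemy message with flat BaseDamage, and BP_BaseEnemy hits also get a movement impulse along fixed X and Z rather than radially.
; The grenade then destroys itself.
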(event `self.Sphere.OnComponentHit`
  (params (HitComponent :type "PrimitiveComponent Object Reference") (OtherActor :type "Actor Object Reference") (OtherComp :type "PrimitiveComponent Object Reference") (NormalImpulse :type "Vector Structure") (Hit :type "HitResult Structure (by ref)"))
  (bind _returnvalue (`self.K2_GetActorLocation`))
  ;[0.4999 0.7026 1] Grenade Impact Damage and Radius
  (if (not (== OtherActor self))
    (bind _outhits (`KismetSystemLibrary.SphereTraceMultiForObjects` _returnvalue (+ _returnvalue (0.0 0.0 0.1)) (`self.Radius`) (`|MakeArray` "ObjectTypeQuery2" "ObjectTypeQuery3" :!type "EObjectTypeQuery Enum") false (`|MakeArray` self :!type "Actor Object Reference") "ForDuration"))
    (for _array_element _outhits
      (bind (_bblockinghit _binitialoverlap _time _distance _location _impactpoint _normal _impactnormal _physmat _hitactor) (`GameplayStatics.BreakHitResult` _array_element))
      (message `/Game/Hordible/Core/AI/BPI_DamageEnemy.DamageEnemy` _hitactor (`self.Base Damage`))
      (bind _asbp_base_enemy (cast `/Game/Hordible/Core/Enemies/BP_BaseEnemy` _hitactor))
      (`CharacterMovementComponent.AddImpulse` (`Character.CharacterMovement` _asbp_base_enemy) (`KismetMathLibrary.MakeVector` (`self.Backwards Impulse`) 0.0 (`self.Upwards Impulse`)) false))
    (`self.K2_DestroyActor`)))

(fn `UserConstructionScript`)
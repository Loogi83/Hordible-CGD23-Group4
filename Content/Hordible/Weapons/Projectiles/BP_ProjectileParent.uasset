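; BP_ProjectileParent is the parent Blueprint for weapon projectiles, exploding on impact to deal area damage.
; When its Sphere component hits something, it spawns a placeholder explosion effect and sphere-traces for Pawn-type objects within the blast radius, with debug drawing left on.
; Each trace hit receives the projectile's full damage, without falloff, plus an ApplyDebuff message, then the projectile destroys itself.
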(event `self.Sphere.OnComponentHit`
  (params (HitComponent :type "PrimitiveComponent Object Reference") (OtherActor :type "Actor Object Reference") (OtherComp :type "PrimitiveComponent Object Reference") (NormalImpulse :type "Vector Structure") (Hit :type "HitResult Structure (by ref)"))
  (bind _returnvalue (`self.K2_GetActorLocation` self))
  (bind _outhits (`KismetSystemLibrary.SphereTraceMultiForObjects` :`Start` _returnvalue :`End` _returnvalue :`Radius` (`self.ProjectileBlastRadius`) :`ObjectTypes` (`|MakeArray` "ObjectTypeQuery3" :!type "EObjectTypeQuery Enum") :`DrawDebugType` "ForDuration"))
  (`NiagaraFunctionLibrary.SpawnSystemAtLocation` "/Game/Hordible/Core/Effects/PS_ExplosionPlaceholder.PS_ExplosionPlaceholder" _returnvalue)
  (for _array_element _outhits
    (bind (_bblockinghit _binitialoverlap _time _distance _location _impactpoint _normal _impactnormal _physmat _hitactor) (`GameplayStatics.BreakHitResult` _array_element))
    (`GameplayStatics.ApplyDamage` _hitactor (`self.ProjectileDamage`))
    (message `/Game/Hordible/Weapons/Projectiles/BPI_AddDebuff.ApplyDebuff` self _hitactor))
  (`self.K2_DestroyActor`))

(fn `UserConstructionScript`)
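; Crossbow weapon Blueprint handling firing, ammo, reloading, and timed infinite-ammo and invisibility-material pickup effects.
; Attack schedules Fire by timer, which multi-line-traces from the arrow along control rotation, spending ammo unless infinite.
; A recoil timeline moves the mesh and damages hit actors on every update, while a reload timeline dips the mesh, then refills ammo.
; StopCharging supports charged shots, but the charge-start logic is disconnected.
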(event `/Game/Hordible/Placeables/Pickups/BPI_PickUp.PickupInvisibility`
  ;[1 1 1] When Invisible Active Set material to Invisible Material
  (`PrimitiveComponent.SetMaterial` (`self.Cube`) 0 "/Game/Hordible/MaterialLibrary/MI_Weapons.MI_Weapons")
  (`KismetSystemLibrary.Delay` 5.0)
  (`PrimitiveComponent.SetMaterial` (`self.Cube`) 0 "/Game/Hordible/MaterialLibrary/M_Weapons.M_Weapons"))

(event `/Game/Hordible/Core/Weapons/BPI_Weapons.InfiniteAmmo`
  (params (Active :type Boolean))
  ;[1 1 1] When Infinite Ammo Active set boolean to true and then to false after 5 seconds
  (set `self.Active` Active)
  (`KismetSystemLibrary.Delay` 5.0)
  (set `self.Active` false))

(event `self.ReceiveBeginPlay`
  (bind _cube (`self.Cube`))
  ;[1 1 1] Set Weapon Location and Rotation
  (set `self.Start Location` (`SceneComponent.RelativeLocation` _cube))
  (set `self.Start Rotation` (`SceneComponent.RelativeRotation` _cube)))

(event `StopCharging`
  ;[0 0.9944 1] Crossbow Charging System For Firing
  (`KismetSystemLibrary.PrintString` "Stop Charging")
  (if (and (`self.IsCharging?`) (>= (`self.CurrentCharge`) 0.2))
    (`self.Fire`))
  (set `self.IsCharging?` false)
  (`TimelineComponent.SetPlayRate` (`self.ChargeWeapon`) 1.0)
  (bind (_direction _charge) (`Timeline|ChargeWeapon` :!via `Reverse`)
    (:`Update`
      (bind _output_get (set `self.CurrentCharge` (`KismetMathLibrary.FClamp` _charge)))
      (if (>= _output_get 1.0)
        (`self.StopCharging`)))))

(event `Reload Icon Anim`
  ;[0 1 0.4738] Crossbow Fire Line Trace
  ;;[1 1 1] Play Reload Icon animation
  (`/Engine/EditorBlueprintResources/StandardMacros.DoOnce` false :!label _label
    (:`Completed`
      (bind _returnvalue (`|CreateWidget` "/Game/Hordible/Core/UI/WBP_ReloadIcon.WBP_ReloadIcon_C"))
      (`UserWidget.AddToViewport` _returnvalue 0))))

(event `self.Manual Reload`
  ;[0 1 0.4738] Crossbow Fire Line Trace
  (`/Engine/EditorBlueprintResources/StandardMacros.DoOnce` false :!label _label_2
    (:`Completed`
      (set `self.CanFire` false)
      (`ActorComponent.Activate` (`self.NS_CrossbowSmoke`) true :!label _label_3)
      (`self.Reload Icon Anim`)
      (`GameplayStatics.PlaySound2D` "/Game/Hordible/Core/Sounds/Nathan/Crossbow_Reload_1_0_Cue_2.Crossbow_Reload_1_0_Cue_2" 1.0 1.0 0.0 null null)
      (bind (_direction _reloadgun) (`Timeline|ReloadingCrossbow` :!via `PlayFromStart`)
        (:`Update`
          (`self.E_ReloadTimer` (`TimelineComponent.GetTimelineLength` (`self.ReloadingCrossbow`)))
          (`SceneComponent.K2_SetRelativeLocation` (`self.Cube`) (`KismetMathLibrary.VLerp` (`self.Start Location`) (- (`self.Start Location`) (`KismetMathLibrary.MakeVector` 0.0 0.0 (`self.TargetReloadLocation`))) _reloadgun) false false))
        (:`Finished`
          (bind _output_get (set `self.Current Ammo` (`self.MaxAmmo`)))
          (set `self.CanFire` true)
          (`self.E_ReduceAmmo` _output_get)
          ;;[1 1 1] Play Reload Icon animation
          (`|ExecutionSequence`
            (:`then_0`
              (goto _label :!via `Reset`))
            (:`then_1`
              (goto _label_2 :!via `Reset`))))))))

(event `self.Attack`
  ;[0 1 0.4738] Crossbow Fire Line Trace
  (if (`self.CanFire`)
    (set `self.CanFire` false)
    (`KismetSystemLibrary.PrintString` (`KismetStringLibrary.Concat_StrStr` "Current Ammo = " (`KismetStringLibrary.Conv_IntToString` (`self.Current Ammo`))) true true (struct :`R` 1.0 :`G` 0.600456 :`A` 1.0) 1.0)
    (if (< (`self.Current Ammo`) 0)
      (goto _label_3)
      (else
        (`GameplayStatics.PlaySound2D` "/Game/Hordible/Core/Sounds/Nathan/Crossbow_Reload_1_0_Cue.Crossbow_Reload_1_0_Cue" 1.0 1.0 0.0 null null)
        (`ActorComponent.Activate` (`self.NS_CrossbowLoadShot`) false)
        (bind _returnvalue (`KismetSystemLibrary.K2_SetTimerDelegate` (delegate `self.Fire`) (`self.CrossBow FireRate`)))
        (set `self.Gun Timer Ref` _returnvalue)
        (`KismetSystemLibrary.K2_SetTimerDelegate` (delegate `Reload`) 0.1 :!label _label_4)))))

(event `self.Fire`
  (bind _start_location (`self.Start Location`))
  (bind _start_rotation (`self.Start Rotation`))
  (bind _returnvalue (`SceneComponent.K2_GetComponentLocation` (`self.Arrow`)))
  ;[0 1 0.4738] Crossbow Fire Line Trace
  (`GameplayStatics.PlaySound2D` "/Game/Hordible/Core/Sounds/Nathan/Crossbow_Firing_1_0_Cue.Crossbow_Firing_1_0_Cue" 1.0 1.0 0.0 null null)
  (if (not (`self.Active`))
    (bind _result (`/Engine/EditorBlueprintResources/StandardMacros.DecrementInt` (`self.Current Ammo`))
      (:`  `
        (`self.E_ReduceAmmo` _result))))
  (`ActorComponent.Activate` (`self.NS_CrossbowFire`) true)
  (bind _outhits (`KismetSystemLibrary.LineTraceMulti` :`Start` _returnvalue :`End` (+ _returnvalue (* (`KismetMathLibrary.GetForwardVector` (`Controller.GetControlRotation` (`GameplayStatics.GetPlayerController` 0))) (`self.TraceRange`))) :`TraceChannel` "TraceTypeQuery4" :`DrawTime` 0.1))
  (bind _asbp_character (cast `/Game/Hordible/Core/Characters/BP_Character` (`GameplayStatics.GetPlayerCharacter` 0)))
  (message `/Game/Hordible/Core/Weapons/BPI_Recoil.Crossbow_Recoil` _asbp_character)
  (bind (_direction _recoil) (`Timeline|Recoil` :!via `PlayFromStart`)
    (:`Update`
      (`SceneComponent.K2_SetRelativeLocationAndRotation` (`self.Cube`) (`KismetMathLibrary.VLerp` _start_location (+ _start_location (-10.0 20.0 15.0)) _recoil) (`KismetMathLibrary.RLerp` _start_rotation (`KismetMathLibrary.ComposeRotators` _start_rotation (struct :`Pitch` 7.0 :`Yaw` 7.0 :`Roll` 2.0)) _recoil true) false false)
      (for _array_element _outhits
        (bind (_bblockinghit _binitialoverlap _time _distance _location _impactpoint _normal _impactnormal _physmat _hitactor) (`GameplayStatics.BreakHitResult` _array_element))
        (message `/Game/Hordible/Core/AI/BPI_DamageEnemy.DamageEnemy` _hitactor (`self.BowDamage`))
        (`KismetSystemLibrary.PrintString` (`KismetSystemLibrary.GetDisplayName` _hitactor)))
      (goto _label_4))))

(event `Reload`
  ;[0 1 0.4738] Crossbow Fire Line Trace
  (set `self.CanFire` true))

(fn `UserConstructionScript`
  (`parent.UserConstructionScript`)
  (set `self.Current Ammo` (`self.maxAmmo`)))
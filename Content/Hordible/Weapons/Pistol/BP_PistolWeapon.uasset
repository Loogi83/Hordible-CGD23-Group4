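; Player pistol weapon that fires hitscan shots, damages what it hits and restores player health on enemy hits.
; Attack gates shots with CanFire and spends ammo, then triggers the line trace on a fire-rate timer or auto-reloads once ammo runs out.
; Timelines animate mesh recoil and reload dip, with Niagara effects on both.
; Pickup events temporarily swap the material for invisibility or suspend ammo use.
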(event `/Game/Hordible/Placeables/Pickups/BPI_PickUp.PickupInvisibility`
  ;[1 1 1] When Invisible Active Set material to Invisible Material
  (`PrimitiveComponent.SetMaterial` (`self.Cube`) 0 "/Game/Hordible/MaterialLibrary/MI_Weapons.MI_Weapons")
  (`KismetSystemLibrary.Delay` 5.0)
  (`PrimitiveComponent.SetMaterial` (`self.Cube`) 0 "/Game/Hordible/MaterialLibrary/M_Weapons.M_Weapons"))

(event `/Game/Hordible/Core/Weapons/BPI_Weapons.InfiniteAmmo`
  (params (Active :type Boolean))
  ;[1 1 1] When Infinite Ammo Active set boolean to true and then to false after 5 seconds
  (set `self.Active` Active)
  (`KismetSystemLibrary.Delay` 5.0)
  (set `self.Active` false))

(event `self.ReceiveBeginPlay`
  (bind _cube (`self.Cube`))
  ;[0.2051 0 0.4072] Set Weapon Location and Rotation
  (set `self.Start Location` (`SceneComponent.RelativeLocation` _cube))
  (set `self.Start Rotation` (`SceneComponent.RelativeRotation` _cube)))

(event `self.Attack`
  (bind _current_ammo (`self.Current Ammo`))
  ;[0.5 0 1] Basic Pistol Fire Functions with Range and Damage Variables
  (if (`self.CanFire`)
    (set `self.CanFire` false)
    (if (not (`self.Active`))
      (`/Engine/EditorBlueprintResources/StandardMacros.DecrementInt` _current_ammo
        (:`  `
          (`KismetSystemLibrary.PrintString` (`KismetStringLibrary.Concat_StrStr` "Current Ammo = " (`KismetStringLibrary.Conv_IntToString` _current_ammo)) true true (struct :`R` 1.0 :`G` 0.613255 :`A` 1.0) 0.1))))
    (if (< (`self.Current Ammo`) 0)
      (`ActorComponent.Activate` (`self.Niagara`) true)
      (bind (_direction _reloadgun) (`Timeline|ReloadTime` :!via `PlayFromStart`)
        (:`Update`
          (`SceneComponent.K2_SetRelativeLocation` (`self.Cube`) (`KismetMathLibrary.VLerp` (`self.Start Location`) (- (`self.Start Location`) (`KismetMathLibrary.MakeVector` 0.0 0.0 (`self.PistolReloadLocation`))) _reloadgun) false false))
        (:`Finished`
          (set `self.Current Ammo` (`self.MaxAmmo`))
          (set `self.CanFire` true)))
      (else
        (`KismetSystemLibrary.K2_SetTimerDelegate` (delegate `self.Fire`) (`self.PistolFireRate`))))))

(event `self.Fire`
  (bind _add_health_to_player (`self.Add Health to Player`))
  (bind _start_location (`self.Start Location`))
  (bind _start_rotation (`self.Start Rotation`))
  (bind _returnvalue (`SceneComponent.K2_GetComponentLocation` (`self.Arrow`)))
  (bind _returnvalue_2 (`Controller.GetControlRotation` (`GameplayStatics.GetPlayerController` 0)))
  ;[0.5 0 1] Basic Pistol Fire Functions with Range and Damage Variables
  (bind _outhit (`KismetSystemLibrary.LineTraceSingle` :`Start` _returnvalue :`End` (+ _returnvalue (* (`KismetMathLibrary.GetForwardVector` _returnvalue_2) (`self.PistolRange`))) :`TraceChannel` "TraceTypeQuery3" :`DrawTime` 0.1))
  (`NiagaraFunctionLibrary.SpawnSystemAtLocation` "/Game/Hordible/Core/Particles/NS_HadesFire.NS_HadesFire" _returnvalue _returnvalue_2)
  (bind _asbp_character (cast `/Game/Hordible/Core/Characters/BP_Character` (`GameplayStatics.GetPlayerCharacter` 0)))
  (message `/Game/Hordible/Core/Weapons/BPI_Recoil.Pistol_Recoil` _asbp_character)
  (bind (_bblockinghit _binitialoverlap _time _distance _location _impactpoint _normal _impactnormal _physmat _hitactor) (`GameplayStatics.BreakHitResult` _outhit))
  (message `/Game/Hordible/Core/AI/BPI_DamageEnemy.DamageEnemy` _hitactor (`self.PistolDamage`))
  (cast `/Game/Hordible/Core/Enemies/BP_BaseEnemy` _hitactor
    (:`then`
      (bind _asbp_character_2 (cast `/Game/Hordible/Core/Characters/BP_Character` (`GameplayStatics.GetPlayerCharacter` 0)))
      (set `/Game/Hordible/Core/Characters/BP_Character.Damage Player` false _asbp_character_2)
      (bind _healthmax (`/Game/Hordible/Core/Characters/BP_Character.HealthMax` _asbp_character_2))
      (if (>= (+ _add_health_to_player (`/Game/Hordible/Core/Characters/BP_Character.HealthCurrent` _asbp_character_2)) _healthmax)
        (set `/Game/Hordible/Core/Characters/BP_Character.HealthCurrent` _healthmax _asbp_character_2)
        (else
          (`/Game/Hordible/Core/Characters/BP_Character.TakeDamage` _asbp_character_2 _add_health_to_player)))
      (set `/Game/Hordible/Core/Characters/BP_Character.Damage Player` true _asbp_character_2))
    (:`CastFailed`
      _))
  (`KismetSystemLibrary.K2_SetTimerDelegate` (delegate `Reload`) (`self.PistolFireRate`))
  (bind (_direction _recoil) (`Timeline|Recoil` :!via `PlayFromStart`)
    (:`Update`
      (`SceneComponent.K2_SetRelativeLocationAndRotation` (`self.Cube`) (`KismetMathLibrary.VLerp` _start_location (+ _start_location (-10.0 20.0 15.0)) _recoil) (`KismetMathLibrary.RLerp` _start_rotation (`KismetMathLibrary.ComposeRotators` _start_rotation (struct :`Pitch` 8.0 :`Yaw` 10.0 :`Roll` 4.0)) _recoil true) false false))))

(event `Reload`
  ;[0.5 0 1] Basic Pistol Fire Functions with Range and Damage Variables
  (set `self.CanFire` true))

(fn `UserConstructionScript`
  (`parent.UserConstructionScript`)
  (set `self.Current Ammo` (`self.MaxAmmo`)))
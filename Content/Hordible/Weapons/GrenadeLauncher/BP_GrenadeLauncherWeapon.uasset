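; Grenade launcher weapon that spawns BP_Grenade from an arrow, with ammo, reloading and timed infinite-ammo and invisibility pickup effects.
; Attack spends ammo and fires, triggering muzzle effects, a character recoil message and timeline-driven gun kick.
; A fire-rate timer then spins the barrel and re-enables firing.
; Dropping below zero ammo, or a manual reload, plays smoke and a gun-lowering timeline that reports reload timing and refills ammo.
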(event `/Game/Hordible/Placeables/Pickups/BPI_PickUp.PickupInvisibility`
  ;[1 1 1] When Invisible Active Set material to Invisible Material
  (`PrimitiveComponent.SetMaterial` (`self.Cube`) 0 "/Game/Hordible/MaterialLibrary/MI_Weapons.MI_Weapons")
  (`KismetSystemLibrary.Delay` 5.0)
  (`PrimitiveComponent.SetMaterial` (`self.Cube`) 0 "/Game/Hordible/MaterialLibrary/M_Weapons.M_Weapons"))

(event `/Game/Hordible/Core/Weapons/BPI_Weapons.InfiniteAmmo`
  (params (Active :type Boolean))
  ;[1 1 1] When Infinite Ammo Active set boolean to true and then to false after 5 seconds
  (set `self.Active` Active)
  (`KismetSystemLibrary.Delay` 5.0)
  (set `self.Active` false))

(event `self.ReceiveBeginPlay`
  (bind _cube (`self.Cube`))
  ;[1 1 1] Set Weapon Location and Rotation
  (set `self.Start Location` (`SceneComponent.RelativeLocation` _cube))
  (set `self.Start Rotation` (`SceneComponent.RelativeRotation` _cube))
  (set `self.Start Rotation_Barrel` (`SceneComponent.RelativeRotation` (`self.Scene`))))

(event `self.Manual Reload`
  ;[1 0 0.75] Grenade Launcher Firing which spawns and fires the grenade actor
  (set `self.CanFire` false)
  (`ActorComponent.Activate` (`self.NS_GrenadeLauncherSmoke`) true :!label _label)
  (bind (_direction _reloadgun) (`Timeline|ReloadingGrenade` :!via `PlayFromStart`)
    (:`Update`
      (`self.E_ReloadTimer` (`TimelineComponent.GetTimelineLength` (`self.ReloadingGrenade`)))
      (`SceneComponent.K2_SetRelativeLocation` (`self.Cube`) (`KismetMathLibrary.VLerp` (`self.Start Location`) (- (`self.Start Location`) (`KismetMathLibrary.MakeVector` 0.0 0.0 (`self.ReloadTargetLocation`))) _reloadgun) false false))
    (:`Finished`
      (bind _output_get (set `self.Current Ammo` (`self.Max Ammo`)))
      (set `self.CanFire` true)
      (`self.E_ReduceAmmo` _output_get))))

(event `self.Attack`
  (bind _current_ammo (`self.Current Ammo`))
  ;[1 0 0.75] Grenade Launcher Firing which spawns and fires the grenade actor
  (if (`self.CanFire`)
    (set `self.CanFire` false)
    (if (not (`self.Active`))
      (`/Engine/EditorBlueprintResources/StandardMacros.DecrementInt` _current_ammo
        (:`  `
          (`self.E_ReduceAmmo` _current_ammo)
          (`KismetSystemLibrary.PrintString` (`KismetStringLibrary.Concat_StrStr` "Current Ammo = " (`KismetStringLibrary.Conv_IntToString` _current_ammo)) true true (struct :`R` 1.0 :`G` 0.585981 :`A` 1.0) 0.5))))
    (if (< (`self.Current Ammo`) 0)
      (goto _label)
      (else
        (`self.Fire`)))))

(event `self.Fire`
  (bind _start_rotation (`self.Start Rotation`))
  (bind _start_location (`self.Start Location`))
  (bind (_returnvalue_location _returnvalue_rotation) (`KismetMathLibrary.BreakTransform` (`SceneComponent.K2_GetComponentToWorld` (`self.Arrow`))))
  ;[1 0 0.75] Grenade Launcher Firing which spawns and fires the grenade actor
  (`|SpawnActorFromClass` "/Game/Hordible/Weapons/Projectiles/BP_Grenade.BP_Grenade_C" (`KismetMathLibrary.MakeTransform` _returnvalue_location _returnvalue_rotation (0.5 0.5 0.5)) "AdjustIfPossibleButAlwaysSpawn" "OverrideRootScale" null null)
  (`NiagaraFunctionLibrary.SpawnSystemAtLocation` "/Game/Hordible/Core/Particles/NS_GrenadeLauncherFire.NS_GrenadeLauncherFire" _returnvalue_location _returnvalue_rotation)
  (bind _asbp_character (cast `/Game/Hordible/Core/Characters/BP_Character` (`GameplayStatics.GetPlayerCharacter` 0)))
  (message `/Game/Hordible/Core/Weapons/BPI_Recoil.Grenade Launcher_Recoil` _asbp_character)
  (`KismetSystemLibrary.K2_SetTimerDelegate` (delegate `Reload`) (`self.LaucherFireRate`))
  (bind (_direction _recoil) (`Timeline|Recoil` :!via `PlayFromStart`)
    (:`Update`
      (`SceneComponent.K2_SetRelativeLocationAndRotation` (`self.Cube`) (`KismetMathLibrary.VLerp` _start_location (+ _start_location (-40.0 25.0 25.0)) _recoil) (`KismetMathLibrary.RLerp` _start_rotation (`KismetMathLibrary.ComposeRotators` _start_rotation (struct :`Pitch` 10.0 :`Yaw` 10.0 :`Roll` 6.0)) _recoil true) false false))))

(event `Reload`
  (bind _start_rotation_barrel (`self.Start Rotation_Barrel`))
  ;[1 0 0.75] Grenade Launcher Firing which spawns and fires the grenade actor
  (bind (_direction _alphacock) (`Timeline|Barrel` :!via `PlayFromStart`)
    (:`Update`
      (bind _output_get (set `self.Start Rotation_Barrel` (`KismetMathLibrary.RLerp` _start_rotation_barrel (`KismetMathLibrary.ComposeRotators` _start_rotation_barrel (struct :`Roll` 10.0)) _alphacock true)))
      (`SceneComponent.K2_SetRelativeRotation` (`self.Scene`) _output_get false false)
      (set `self.CanFire` true))))

(fn `UserConstructionScript`
  (`parent.UserConstructionScript`)
  (set `self.Current Ammo` (`self.Max Ammo`)))
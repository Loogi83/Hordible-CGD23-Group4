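; Bloblin enemy that splits into a number of smaller Bloblet enemies when it dies.
; Its Death override disables collision, then spawns each Bloblet at the BlobletSpawn component and registers it with the Manager as an enemy.
; Each valid Bloblet is launched upward with random horizontal velocity to scatter the group, then the parent death logic runs.
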(fn `Death`
  (bind _returnvalue (`KismetMathLibrary.RandomFloatInRange` -300.0 300.0))
  (bind _returnvalue_location (`KismetMathLibrary.BreakTransform` (`SceneComponent.K2_GetComponentToWorld` (`self.BlobletSpawn`))))
  ;[1 1 1] spawns x number of enemies at Bloblin location on death
  (`self.SetActorEnableCollision` self false)
  (for _ (range 1 (+ (`self.NumberOfEnemiesToSpawn`) 1))
    (bind _returnvalue_2 (`|SpawnActorFromClass` "/Game/Hordible/Enemies/EnemyTypes/Bloblet/BP_Bloblet.BP_Bloblet_C" (`KismetMathLibrary.MakeTransform` _returnvalue_location) "AdjustIfPossibleButAlwaysSpawn" "OverrideRootScale" null null))
    (`/Game/Hordible/Core/Managers/BP_WaveManager.AddEnemy` (`self.Manager`) _returnvalue_2)
    (`/Engine/EditorBlueprintResources/StandardMacros.IsValid` _returnvalue_2
      (:`Is Valid`
        (`self.LaunchCharacter` _returnvalue_2 (`KismetMathLibrary.MakeVector` _returnvalue _returnvalue 200.0) false false))))
  (`parent.Death`))

(fn `UserConstructionScript`
  (`parent.UserConstructionScript`))
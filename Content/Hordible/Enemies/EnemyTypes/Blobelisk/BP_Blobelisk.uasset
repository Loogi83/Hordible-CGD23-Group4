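; Blobelisk enemy that turns toward the player inside its attack-range sphere and damages them on contact with its box collision.
; Entering range starts a looping detection timer, yaws the body toward the player and pitches the projectile-spawn arrow; leaving clears the timers.
; A stats struct drives health, speed, range and damage, with death signalling a kill and destroying the actor.
; FireProjectile spawns a projectile from the arrow, but nothing here calls it.
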(event `self.Collision_AttackRange.OnComponentBeginOverlap`
  (params (OverlappedComponent :type "PrimitiveComponent Object Reference") (OtherActor :type "Actor Object Reference") (OtherComp :type "PrimitiveComponent Object Reference") (OtherBodyIndex :type Integer) (bFromSweep :type Boolean) (SweepResult :type "HitResult Structure (by ref)"))
  ;[1 1 1] Start/Stop firing on collision with attack radius
  (cast `/Game/Hordible/Core/Characters/BP_Character` OtherActor)
  (set `self.PlayerInRange` true)
  (`self.FacePlayer`))

(event `FacePlayer`
  (bind (_returnvalue_roll _returnvalue_pitch) (`KismetMathLibrary.BreakRotator` (`KismetMathLibrary.FindLookAtRotation` (`SceneComponent.K2_GetComponentLocation` (`self.DirectionalArrow`)) (`self.K2_GetActorLocation` (`GameplayStatics.GetPlayerCharacter` 0)))))
  ;[1 0.4271 0.4271] FacePlayerEvent
  ;;[1 0.4271 0.4271] Rotate Mesh to Player
  (bind _returnvalue (`KismetSystemLibrary.K2_SetTimerDelegate` (`|CreateDelegate` :!event `FacePlayer`) 0.02 true))
  (set `self.DetectionTimer` _returnvalue)
  (`self.Rotate to Player`)
  ;;[1 0.4271 0.4271] Rotate arrow (projectile spawner) to face player
  (`SceneComponent.K2_SetRelativeRotation` (`self.DirectionalArrow`) (`KismetMathLibrary.MakeRotator` 0.0 (+ _returnvalue_pitch 7.0)) false false))

(event `self.Collision_AttackRange.OnComponentEndOverlap`
  (params (OverlappedComponent :type "PrimitiveComponent Object Reference") (OtherActor :type "Actor Object Reference") (OtherComp :type "PrimitiveComponent Object Reference") (OtherBodyIndex :type Integer))
  ;[1 1 1] Start/Stop firing on collision with attack radius
  (cast `/Game/Hordible/Core/Characters/BP_Character` OtherActor)
  (set `self.PlayerInRange` false)
  (`KismetSystemLibrary.K2_ClearAndInvalidateTimerHandle` (`self.FireTimer`))
  (`KismetSystemLibrary.K2_ClearAndInvalidateTimerHandle` (`self.DetectionTimer`)))

(event `/Game/Hordible/Core/AI/BPI_DamageEnemy.DamageEnemy`
  (params (DamageToDeal :type "Float (double-precision)"))
  ;[1 1 1] Take Damage
  (`self.TakeDamage` DamageToDeal))

(event `self.ReceiveTick`
  (params (DeltaSeconds :type "Float (single-precision)"))
  ;[1 1 1] Debug stats
  (`KismetSystemLibrary.DrawDebugString` (0.0 0.0 100.0) (`KismetStringLibrary.Conv_DoubleToString` (`.CurrentHealth_4_84644DB54A34569CA27C329BDE205092` (break `/Game/Hordible/Core/Enemies/S_EnemyStats` (`self.Stats`)))) self (struct :`A` 1.0)))

(event `self.BoxCollision.OnComponentBeginOverlap`
  (params (OverlappedComponent :type "PrimitiveComponent Object Reference") (OtherActor :type "Actor Object Reference") (OtherComp :type "PrimitiveComponent Object Reference") (OtherBodyIndex :type Integer) (bFromSweep :type Boolean) (SweepResult :type "HitResult Structure (by ref)"))
  ;[1 1 1] Damage player on overlap with blobalisk mesh
  (bind _asbp_character (cast `/Game/Hordible/Core/Characters/BP_Character` OtherActor))
  (`/Game/Hordible/Core/Characters/BP_Character.TakeDamage` _asbp_character (`.Damage_8_A59EF6524CE3ECB8D33F908D74FB7CE2` (break `/Game/Hordible/Core/Enemies/S_EnemyStats` (`self.Stats`)))))

(event `self.BoxCollision.OnComponentEndOverlap`
  (params (OverlappedComponent :type "PrimitiveComponent Object Reference") (OtherActor :type "Actor Object Reference") (OtherComp :type "PrimitiveComponent Object Reference") (OtherBodyIndex :type Integer))
  ;[1 1 1] Damage player on overlap with blobalisk mesh
  (cast `/Game/Hordible/Core/Characters/BP_Character` OtherActor))

(fn `Death`
  (`KismetSystemLibrary.PrintString` (`KismetStringLibrary.Concat_StrStr` (`KismetSystemLibrary.GetDisplayName` self) " has died!"))
  (`self.K2_DestroyActor`))

(fn `FireProjectile`
  (bind (_returnvalue_location _returnvalue_rotation) (`KismetMathLibrary.BreakTransform` (`SceneComponent.K2_GetComponentToWorld` (`self.DirectionalArrow`))))
  (`|SpawnActorFromClass` "/Game/Hordible/Weapons/Projectiles/BP_ProjectileParent.BP_ProjectileParent_C" (`KismetMathLibrary.MakeTransform` _returnvalue_location _returnvalue_rotation (`self.ProjectileScale`)) "AdjustIfPossibleButAlwaysSpawn" "OverrideRootScale" null null))

(fn `Rotate to Player`
  (bind (_returnvalue_roll _returnvalue_pitch _returnvalue_yaw) (`KismetMathLibrary.BreakRotator` (`KismetMathLibrary.RInterpTo` (`self.K2_GetActorRotation` self) (`KismetMathLibrary.FindLookAtRotation` (`self.K2_GetActorLocation` self) (`self.K2_GetActorLocation` (`GameplayStatics.GetPlayerCharacter` 0))) (`GameplayStatics.GetWorldDeltaSeconds`) 20.0)))
  (`self.K2_SetActorRotation` self (`KismetMathLibrary.MakeRotator` 0.0 0.0 _returnvalue_yaw) false))

(fn `TakeDamage`
  (params (DamageDealt :type "Float (double-precision)"))
  (bind (_movementspeed _currenthealth) (break `/Game/Hordible/Core/Enemies/S_EnemyStats` (`self.Stats`)))
  (setmembers `/Game/Hordible/Core/Enemies/S_EnemyStats` :`StructRef` (`self.Stats`) :`CurrentHealth` (- _currenthealth DamageDealt))
  (if (<= _currenthealth 0.0)
    (`self.EEnemyKilled`)
    (`self.Death`)))

(fn `UserConstructionScript`
  (bind _stats (`self.Stats`))
  (bind ((`MovementSpeed_2_28FA2C6348DBB2A1392799B2F3D03407` _movementspeed) (`MaxHealth_6_D9738A614FE71AD569592B8B8F0B25C8` _maxhealth)) (break `/Game/Hordible/Core/Enemies/S_EnemyStats` _stats))
  ;[1 1 1] Sets current health to max (saves manually changing both stats)
  (setmembers `/Game/Hordible/Core/Enemies/S_EnemyStats` :`StructRef` _stats :`CurrentHealth` _maxhealth)
  ;[1 1 1] Sets character movement speed as struct variable
  (set `CharacterMovementComponent.MaxWalkSpeed` _movementspeed (`self.CharacterMovement`))
  (`SphereComponent.SetSphereRadius` (`self.Collision_AttackRange`) (`.Range_10_B15BB72946686B2C2C713B9A915B6090` (break `/Game/Hordible/Core/Enemies/S_EnemyStats` (`self.Stats`))) true))
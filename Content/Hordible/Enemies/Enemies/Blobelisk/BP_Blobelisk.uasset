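; Blobelisk enemy with a pillar mesh that tracks the player within its Stats-driven attack radius and damages them on contact.
; Entering range starts a looping timer and turns the mesh and projectile-spawn arrow toward the player; leaving clears detection and fire timers.
; FireProjectile spawns debuff projectiles from the arrow, though nothing here calls it.
; Damage raises enemy events and lowers health, ending in death effects and destruction.
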(event `self.ReceiveBeginPlay`
  (add `self.EEnemyDamaged` (`|CreateDelegate` :!event `SpawnDamagePopup`)))

(event `self.Collision_AttackRange.OnComponentBeginOverlap`
  (params (OverlappedComponent :type "PrimitiveComponent Object Reference") (OtherActor :type "Actor Object Reference") (OtherComp :type "PrimitiveComponent Object Reference") (OtherBodyIndex :type Integer) (bFromSweep :type Boolean) (SweepResult :type "HitResult Structure (by ref)"))
  ;[1 1 1] Start/Stop firing on collision with attack radius
  (cast `/Game/Hordible/Core/Characters/BP_Character` OtherActor)
  (set `self.PlayerInRange` true)
  (`self.FacePlayer`))

(event `FacePlayer`
  ;[1 0.4271 0.4271] FacePlayerEvent
  ;;[1 0.4271 0.4271] Rotate Mesh to Player
  (bind _returnvalue (`KismetSystemLibrary.K2_SetTimerDelegate` (`|CreateDelegate` :!event `FacePlayer`) 0.02 true))
  (set `self.DetectionTimer` _returnvalue)
  (`self.Rotate to Player`))

(event `self.Collision_AttackRange.OnComponentEndOverlap`
  (params (OverlappedComponent :type "PrimitiveComponent Object Reference") (OtherActor :type "Actor Object Reference") (OtherComp :type "PrimitiveComponent Object Reference") (OtherBodyIndex :type Integer))
  ;[1 1 1] Start/Stop firing on collision with attack radius
  (cast `/Game/Hordible/Core/Characters/BP_Character` OtherActor)
  (set `self.PlayerInRange` false)
  (`KismetSystemLibrary.K2_ClearAndInvalidateTimerHandle` (`self.FireTimer`))
  (`KismetSystemLibrary.K2_ClearAndInvalidateTimerHandle` (`self.DetectionTimer`)))

(event `SpawnDamagePopup` :!signature `self.EEnemyDamaged`
  (params (Amount :type "Float (double-precision)"))
  ;[1 1 1] Cheeky bit of UI for damage stats
  (`|SpawnActorFromClass` "/Game/Hordible/Core/UI/PopupTextWidgets/BP_TextPopup.BP_TextPopup_C" (`KismetMathLibrary.MakeTransform` (`self.K2_GetActorLocation`)) "Undefined" "OverrideRootScale" null (`KismetStringLibrary.Conv_DoubleToString` Amount) (struct :`R` 1.0 :`G` 0.012647 :`A` 1.0) null)
  (`KismetSystemLibrary.PrintString` "Damaging Enemy"))

(event `/Game/Hordible/Core/AI/BPI_DamageEnemy.DamageEnemy`
  (params (DamageToDeal :type "Float (double-precision)"))
  ;[1 1 1] Take Damage
  (`self.TakeDamage` DamageToDeal))

(event `self.ReceiveTick`
  (params (DeltaSeconds :type "Float (single-precision)"))
  ;[1 1 1] Debug stats
  (`KismetSystemLibrary.DrawDebugString` (0.0 0.0 100.0) (`KismetStringLibrary.Conv_DoubleToString` (`.CurrentHealth_4_84644DB54A34569CA27C329BDE205092` (break `/Game/Hordible/Core/Enemies/S_EnemyStats` (`self.Stats`)))) self (struct :`A` 1.0)))

(event `self.BoxCollision.OnComponentBeginOverlap`
  (params (OverlappedComponent :type "PrimitiveComponent Object Reference") (OtherActor :type "Actor Object Reference") (OtherComp :type "PrimitiveComponent Object Reference") (OtherBodyIndex :type Integer) (bFromSweep :type Boolean) (SweepResult :type "HitResult Structure (by ref)"))
  ;[1 1 1] Damage player on overlap with blobalisk mesh
  (bind _asbp_character (cast `/Game/Hordible/Core/Characters/BP_Character` OtherActor))
  (`/Game/Hordible/Core/Characters/BP_Character.TakeDamage` _asbp_character (`.Damage_8_A59EF6524CE3ECB8D33F908D74FB7CE2` (break `/Game/Hordible/Core/Enemies/S_EnemyStats` (`self.Stats`)))))

(event `self.BoxCollision.OnComponentEndOverlap`
  (params (OverlappedComponent :type "PrimitiveComponent Object Reference") (OtherActor :type "Actor Object Reference") (OtherComp :type "PrimitiveComponent Object Reference") (OtherBodyIndex :type Integer))
  ;[1 1 1] Damage player on overlap with blobalisk mesh
  (cast `/Game/Hordible/Core/Characters/BP_Character` OtherActor))

(fn `Death`
  (`NiagaraFunctionLibrary.SpawnSystemAtLocation` "/Game/Hordible/Enemies/Enemies/PS_EnemyDeath.PS_EnemyDeath" (+ (`SceneComponent.K2_GetComponentLocation` (`self.Mesh`)) (0.0 0.0 100.0)))
  (`NiagaraFunctionLibrary.SpawnSystemAtLocation` "/Game/Hordible/Enemies/Enemies/PS_PillarDeath.PS_PillarDeath" (`SceneComponent.K2_GetComponentLocation` (`self.SM_Pillar`)))
  (`self.K2_DestroyActor`))

(fn `FireProjectile`
  (bind (_returnvalue_location _returnvalue_rotation) (`KismetMathLibrary.BreakTransform` (`SceneComponent.K2_GetComponentToWorld` (`self.DirectionalArrow`))))
  (`|SpawnActorFromClass` "/Game/Hordible/Weapons/Projectiles/BP_DebuffProjectile.BP_DebuffProjectile_C" (`KismetMathLibrary.MakeTransform` _returnvalue_location _returnvalue_rotation (`self.ProjectileScale`)) "AdjustIfPossibleButAlwaysSpawn" "OverrideRootScale" null 0.0 self))

(fn `Rotate to Player`
  (bind _mesh (`self.Mesh`))
  (bind _directionalarrow (`self.DirectionalArrow`))
  (bind (_returnvalue_roll _returnvalue_pitch _returnvalue_yaw) (`KismetMathLibrary.BreakRotator` (`KismetMathLibrary.FindLookAtRotation` (`SceneComponent.K2_GetComponentLocation` _directionalarrow) (`self.K2_GetActorLocation` (`GameplayStatics.GetPlayerCharacter` 0)))))
  (bind (_returnvalue_roll_2 _returnvalue_pitch_2 _returnvalue_yaw_2) (`KismetMathLibrary.BreakRotator` (`KismetMathLibrary.RInterpTo` (`SceneComponent.K2_GetComponentRotation` _mesh) (`KismetMathLibrary.ComposeRotators` (`KismetMathLibrary.FindLookAtRotation` (`SceneComponent.K2_GetComponentLocation` _mesh) (`self.K2_GetActorLocation` (`GameplayStatics.GetPlayerCharacter` 0))) (struct :`Yaw` -90.0)) (`GameplayStatics.GetWorldDeltaSeconds`) 20.0)))
  ;[1 1 1] rotates mesh to face player
  (`SceneComponent.K2_SetWorldRotation` (`self.Mesh`) (`KismetMathLibrary.MakeRotator` 0.0 0.0 _returnvalue_yaw_2) false false)
  ;[1 1 1] Controls pitch so directional arrow (projectile spawner) points at player
  (`SceneComponent.K2_SetWorldRotation` _directionalarrow (`KismetMathLibrary.MakeRotator` _returnvalue_roll (+ _returnvalue_pitch 10.0) _returnvalue_yaw) false false))

(fn `TakeDamage`
  (params (DamageDealt :type "Float (double-precision)"))
  (bind (_movementspeed _currenthealth) (break `/Game/Hordible/Core/Enemies/S_EnemyStats` (`self.Stats`)))
  (`self.EEnemyDamaged` DamageDealt)
  (setmembers `/Game/Hordible/Core/Enemies/S_EnemyStats` :`StructRef` (`self.Stats`) :`CurrentHealth` (- _currenthealth DamageDealt))
  (if (<= _currenthealth 0.0)
    (`self.EEnemyKilled` 0.0)
    (`KismetSystemLibrary.PrintString` "Blobelisk Killed")
    (`self.Death`)))

(fn `UserConstructionScript`
  (bind _stats (`self.Stats`))
  (bind ((`MovementSpeed_2_28FA2C6348DBB2A1392799B2F3D03407` _movementspeed) (`MaxHealth_6_D9738A614FE71AD569592B8B8F0B25C8` _maxhealth)) (break `/Game/Hordible/Core/Enemies/S_EnemyStats` _stats))
  ;[1 1 1] Sets current health to max (saves manually changing both stats)
  (setmembers `/Game/Hordible/Core/Enemies/S_EnemyStats` :`StructRef` _stats :`CurrentHealth` _maxhealth)
  ;[1 1 1] Sets character movement speed as struct variable
  (set `CharacterMovementComponent.MaxWalkSpeed` _movementspeed (`self.CharacterMovement`))
  (`SphereComponent.SetSphereRadius` (`self.Collision_AttackRange`) (`.Range_10_B15BB72946686B2C2C713B9A915B6090` (break `/Game/Hordible/Core/Enemies/S_EnemyStats` (`self.Stats`))) true))
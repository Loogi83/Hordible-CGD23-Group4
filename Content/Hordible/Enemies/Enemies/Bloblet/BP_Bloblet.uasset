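; BP_Bloblet is the Bloblet enemy, a child Blueprint that adds a melee attack against the player character.
; An AttackRig event toggles the attack window, and MeleeCollision overlaps with BP_Character during it send the Stats damage through DamagePlayerMessage.
; A DoOnce limits each window to one hit, clearing the active flag on contact and resetting when the rig switches off.
; Death and construction only call the parent.
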(event `self.MeleeCollision.OnComponentBeginOverlap`
  (params (OverlappedComponent :type "PrimitiveComponent Object Reference") (OtherActor :type "Actor Object Reference") (OtherComp :type "PrimitiveComponent Object Reference") (OtherBodyIndex :type Integer) (bFromSweep :type Boolean) (SweepResult :type "HitResult Structure (by ref)"))
  ;[1 1 1] Apply Damage if attack rig is active - switch off after damage is applied then reset when it's switched off
  (cast `/Game/Hordible/Core/Characters/BP_Character` OtherActor)
  (if (`self.AttackActive`)
    (`/Engine/EditorBlueprintResources/StandardMacros.DoOnce` false :!label _label
      (:`Completed`
        (set `self.AttackActive` false)
        (message `/Game/Hordible/Core/Characters/BPI_DamagePlayer.DamagePlayer` OtherActor (`.Damage_8_A59EF6524CE3ECB8D33F908D74FB7CE2` (break `/Game/Hordible/Core/Enemies/S_EnemyStats` (`self.Stats`))))))))

(event `AttackRig`
  (params (`Rig Active?` :type Boolean))
  ;[1 1 1] Apply Damage if attack rig is active - switch off after damage is applied then reset when it's switched off
  (bind _output_get (set `self.AttackActive` `Rig Active?`))
  (if (not _output_get)
    (goto _label :!via `Reset`)))

(fn `Death`
  (`parent.Death`))

(fn `UserConstructionScript`
  (`parent.UserConstructionScript`))
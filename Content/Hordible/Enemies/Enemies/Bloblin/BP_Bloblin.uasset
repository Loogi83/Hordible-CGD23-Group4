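; Bloblin melee enemy that knocks the player back and splits into smaller Bloblets on death.
; AttackCollision toggles the attack window and re-arms a DoOnce, so the hitbox overlap deals damage once per attack, plus an impulse along the player mesh's reversed forward vector and upward.
; Death override plays an effect, launches Bloblets in random directions and registers them with Manager before calling the parent.
; DustPS spawns dust at the hand socket.
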(event `self.ReceiveTick`
  (params (DeltaSeconds :type "Float (single-precision)"))
  (`parent.ReceiveTick` DeltaSeconds))

(event `self.Collision_Attack.OnComponentBeginOverlap`
  (params (OverlappedComponent :type "PrimitiveComponent Object Reference") (OtherActor :type "Actor Object Reference") (OtherComp :type "PrimitiveComponent Object Reference") (OtherBodyIndex :type Integer) (bFromSweep :type Boolean) (SweepResult :type "HitResult Structure (by ref)"))
  ;[1 1 1] Apply damage to player if MeleeCollision hits Player & attack active is true
  (bind _asbp_character (cast `/Game/Hordible/Core/Characters/BP_Character` OtherActor))
  (if (`self.AttackActive`)
    (`/Engine/EditorBlueprintResources/StandardMacros.DoOnce` false :!label _label
      (:`Completed`
        (set `self.AttackActive` false)
        (message `/Game/Hordible/Core/Characters/BPI_DamagePlayer.DamagePlayer` _asbp_character (`.Damage_8_A59EF6524CE3ECB8D33F908D74FB7CE2` (break `/Game/Hordible/Core/Enemies/S_EnemyStats` (`self.Stats`))))
        ;[1 1 1] Adds impulse to player - will optimise this in future
        (bind _asbp_character_2 (cast `/Game/Hordible/Core/Characters/BP_Character` (`GameplayStatics.GetPlayerCharacter` 0)))
        (bind (_returnvalue_x _returnvalue_y) (`KismetMathLibrary.BreakVector` (* (`SceneComponent.GetForwardVector` (`Character.Mesh` _asbp_character_2)) -50000.0)))
        (`CharacterMovementComponent.AddImpulse` (`Character.CharacterMovement` _asbp_character_2) (`KismetMathLibrary.MakeVector` _returnvalue_x _returnvalue_y 50000.0) false)))))

(event `AttackCollision`
  (params (Enabled :type Boolean))
  ;[1 1 1] Apply damage to player if MeleeCollision hits Player & attack active is true
  (bind _output_get (set `self.AttackActive` Enabled))
  (if (not _output_get)
    (goto _label :!via `Reset`)))

(fn `Death`
  (bind _returnvalue (`KismetMathLibrary.RandomFloatInRange` -300.0 300.0))
  (bind _returnvalue_location (`KismetMathLibrary.BreakTransform` (`SceneComponent.K2_GetComponentToWorld` (`self.BlobletSpawn`))))
  (if (`self.NowDie`)
    (`NiagaraFunctionLibrary.SpawnSystemAtLocation` "/Game/Hordible/Enemies/Enemies/PS_EnemyDeath.PS_EnemyDeath" (`self.K2_GetActorLocation` self))
    ;[1 1 1] spawns x number of enemies at Bloblin location on death
    (`self.SetActorEnableCollision` self false)
    (for _ (range 1 (+ (`self.NumberOfEnemiesToSpawn`) 1))
      (bind _returnvalue_2 (`|SpawnActorFromClass` "/Game/Hordible/Enemies/Enemies/Bloblet/BP_Bloblet.BP_Bloblet_C" (`KismetMathLibrary.MakeTransform` (`KismetMathLibrary.RandomPointInBoundingBox` _returnvalue_location (5.0 5.0 5.0))) "AdjustIfPossibleButDontSpawnIfColliding" "OverrideRootScale" null null))
      (`/Game/Hordible/Core/Managers/BP_WaveManager.AddEnemy` (`self.Manager`) _returnvalue_2)
      (`/Engine/EditorBlueprintResources/StandardMacros.IsValid` _returnvalue_2
        (:`Is Valid`
          (`self.LaunchCharacter` _returnvalue_2 (`KismetMathLibrary.MakeVector` _returnvalue _returnvalue 200.0) false false))))
    (`parent.Death`)))

(fn `DustPS`
  (`NiagaraFunctionLibrary.SpawnSystemAtLocation` "/Game/Hordible/Art/Particles/Dust_2_System.Dust_2_System" (`SceneComponent.GetSocketLocation` (`self.Mesh`) "Socket_Hand")))

(fn `UserConstructionScript`
  (`parent.UserConstructionScript`))
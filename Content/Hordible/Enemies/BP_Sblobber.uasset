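; BP_Sblobber is a Hordible enemy that signals its AI to retreat when the player character gets too close.
; Entering the fallback sphere sets the Retreat blackboard key, and only leaving the larger attack sphere clears it, giving the retreat hysteresis.
; Construction sizes the attack sphere from the Range stat and the fallback sphere from that range minus a margin, passed through a clamp.
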(event `self.Collision_FallBackRange.OnComponentBeginOverlap`
  (params (OverlappedComponent :type "PrimitiveComponent Object Reference") (OtherActor :type "Actor Object Reference") (OtherComp :type "PrimitiveComponent Object Reference") (OtherBodyIndex :type Integer) (bFromSweep :type Boolean) (SweepResult :type "HitResult Structure (by ref)"))
  ;[1 1 1] Set Retreat Key / Start Retreat Sequence
  (cast `/Game/Hordible/Core/Characters/BP_Character` OtherActor)
  (`BlackboardComponent.SetValueAsBool` (`AIController.Blackboard` (`AIBlueprintHelperLibrary.GetAIController` self)) "Retreat" true))

(event `self.Collision_AttackRange.OnComponentEndOverlap`
  (params (OverlappedComponent :type "PrimitiveComponent Object Reference") (OtherActor :type "Actor Object Reference") (OtherComp :type "PrimitiveComponent Object Reference") (OtherBodyIndex :type Integer))
  ;[1 1 1] Clear Retreat Key / Stop Retreat Sequence
  (cast `/Game/Hordible/Core/Characters/BP_Character` OtherActor)
  (`BlackboardComponent.ClearValue` (`AIController.Blackboard` (`AIBlueprintHelperLibrary.GetAIController` self)) "Retreat"))

(fn `UserConstructionScript`
  (bind ((`Range_10_B15BB72946686B2C2C713B9A915B6090` _range)) (break `/Game/Hordible/Core/Enemies/S_EnemyStats` (`self.Stats`)))
  (bind _returnvalue (- _range 200.0))
  (`parent.UserConstructionScript`)
  (`SphereComponent.SetSphereRadius` (`self.Collision_AttackRange`) _range true)
  (`SphereComponent.SetSphereRadius` (`self.Collision_FallBackRange`) (`KismetMathLibrary.FClamp` _returnvalue 300.0 _returnvalue) true))